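; Mission spawner actor that creates a NavePlaceholder ship carrying a pickable Dynamite.
; SpawnPlaceholder runs once, spawning the ship at the spawner's transform and copying its waypoint and movement settings onto it.
; It then spawns Dynamite at the ship's dynamite spawn location and attaches it to the Dynamite socket.
; The dynamite's OnPicked event is re-broadcast through the spawner's own OnDynamitePicked dispatcher.
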(event Custom|SpawnPlaceholder
  (Utilities|FlowControl|DoOnce false
    (:Completed
      (bind _returnvalue (Game|SpawnActorfromClass "/Game/Blueprints/Mission/NavePlaceholder.NavePlaceholder_C" (Transformation|GetWorldTransform (Variables|Default|GetDefaultSceneRoot)) "AlwaysSpawn" 0 0))
      (Variables|Default|SetPlaceholderSpawned _returnvalue)
      (Variables|/Game/Blueprints/Mission/NavePlaceholder.NavePlaceholder_C|SetWaypoints (Variables|Default|GetPlaceholderSpawned) (Variables|Default|GetWaypoints))
      (Variables|/Game/Blueprints/Mission/NavePlaceholder.NavePlaceholder_C|SetCurrentWaypoint (Variables|Default|GetPlaceholderSpawned) (Variables|Default|GetCurrentWaypoint))
      (Variables|/Game/Blueprints/Mission/NavePlaceholder.NavePlaceholder_C|SetDistanceToGoal (Variables|Default|GetPlaceholderSpawned) (Variables|Default|GetDistanceToGoal))
      (Variables|/Game/Blueprints/Mission/NavePlaceholder.NavePlaceholder_C|SetSpeed (Variables|Default|GetPlaceholderSpawned) (Variables|Default|GetSpeed))
      (Variables|/Game/Blueprints/Mission/NavePlaceholder.NavePlaceholder_C|SetVelocidadDeGiro (Variables|Default|GetPlaceholderSpawned) (Variables|Default|GetVelocidadDeGiro))
      (bind _spawnlocation (Default|GetDynamiteSpawnLocation (Variables|Default|GetPlaceholderSpawned)))
      (bind _returnvalue_2 (Game|SpawnActorfromClass "/Game/Blueprints/Objects/Dynamite.Dynamite_C" (Math|Transform|MakeTransform _spawnlocation (Transformation|GetWorldRotation (Variables|Default|GetDefaultSceneRoot)) "1,1,1") "AlwaysSpawn" 0 0))
      (Transformation|AttachActorToActor _returnvalue_2 (Variables|Default|GetPlaceholderSpawned) "Dynamite" "KeepWorld" "KeepRelative" "KeepWorld" true)
      (EventDispatchers|BindEventtoOnPicked _returnvalue_2 (delegate Custom|PickedDynamite)))))

(event Custom|PickedDynamite
  (Default|CallOnDynamitePicked))

(fn ConstructionScript)