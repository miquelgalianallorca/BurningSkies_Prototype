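; Placeholder ship actor for a mission that flies along an array of waypoint actors, then destroys itself after the last one.
; Tick moves it without sweep and eases its rotation toward the current waypoint, jumping to high speed with trigger collision off on the final leg.
; A player entering or leaving its sphere switches speed between faster and slower values.
; The construction script draws the route as debug lines, and a function exposes a dynamite spawn point.
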(event OnComponentBeginOverlap(Sphere)
  (params (OverlappedComponent :type Primitive%20Component%20Object%20Reference) (OtherActor :type Actor%20Object%20Reference) (OtherComp :type Primitive%20Component%20Object%20Reference) (OtherBodyIndex :type Integer) (bFromSweep :type Boolean) (SweepResult :type Hit%20Result%20Structure%20%28by%20ref%29))
  (Utilities|Casting|CastToPlayerCharacter OtherActor)
  (Variables|Default|SetSpeed (Math|Float|Lerp (Variables|Default|GetSpeed) 3.5e+03 1.0)))

(event OnComponentBeginOverlap(Box)
  (params (OverlappedComponent :type Primitive%20Component%20Object%20Reference) (OtherActor :type Actor%20Object%20Reference) (OtherComp :type Primitive%20Component%20Object%20Reference) (OtherBodyIndex :type Integer) (bFromSweep :type Boolean) (SweepResult :type Hit%20Result%20Structure%20%28by%20ref%29)))

(event OnComponentEndOverlap(Sphere)
  (params (OverlappedComponent :type Primitive%20Component%20Object%20Reference) (OtherActor :type Actor%20Object%20Reference) (OtherComp :type Primitive%20Component%20Object%20Reference) (OtherBodyIndex :type Integer))
  (Utilities|Casting|CastToPlayerCharacter OtherActor)
  (Variables|Default|SetSpeed (Math|Float|Lerp (Variables|Default|GetSpeed) 2.5e+03 1.0)))

(event EventBeginPlay)

(event Collision|EventActorBeginOverlap
  (params (OtherActor :type Actor%20Object%20Reference)))

(event EventTick
  (params (DeltaSeconds :type Float%20%28single-precision%29))
  (bind _returnvalue (Transformation|GetActorLocation))
  (bind _waypoints (Variables|Default|GetWaypoints))
  (if (< (Variables|Default|GetCurrentWaypoint) (Utilities|Array|Length _waypoints))
    (if (> (Math|Vector|VectorLength (- (Transformation|GetActorLocation (Utilities|Array|Get(acopy) _waypoints (Variables|Default|GetCurrentWaypoint))) _returnvalue)) (Variables|Default|GetDistanceToGoal))
      (Transformation|SetActorLocation (+ _returnvalue (* (Math|Vector|Normalize (- (Transformation|GetActorLocation (Utilities|Array|Get(acopy) _waypoints (Variables|Default|GetCurrentWaypoint))) _returnvalue)) (* (Variables|Default|GetSpeed) DeltaSeconds))) false false)
      (Transformation|SetActorRotation (Math|Rotator|Lerp(Rotator) (Transformation|GetActorRotation) (Math|Rotator|FindLookatRotation _returnvalue (Transformation|GetActorLocation (Utilities|Array|Get(acopy) _waypoints (Variables|Default|GetCurrentWaypoint)))) (* DeltaSeconds (Variables|Default|GetVelocidadDeGiro)) true))
      (if (== (Variables|Default|GetCurrentWaypoint) (- (Utilities|Array|Length (Variables|Default|GetWaypoints)) 1))
        (Variables|Default|SetSpeed (Math|Float|Lerp (Variables|Default|GetSpeed) 8e+03 1.0))
        (Collision|SetCollisionEnabled (Variables|Default|GetSphere) "NoCollision"))
      (else
        (bind _result (Math|Integer|IncrementInt (Variables|Default|GetCurrentWaypoint))
          (:%20%20
            (Variables|Default|SetCurrentWaypoint _result)))))
    (else
      (Actor|DestroyActor))))

(fn ConstructionScript
  (for (_array_element _array_index) (Variables|Default|GetWaypoints)
    (if (< (+ _array_index 1) (Utilities|Array|Length (Variables|Default|GetWaypoints)))
      (Rendering|Debug|DrawDebugLine (Transformation|GetActorLocation _array_element) (Transformation|GetActorLocation (Utilities|Array|Get(acopy) (Variables|Default|GetWaypoints) (+ _array_index 1))) "(R=1.000000,G=0.017847,B=0.000000,A=1.000000)" 1.2e+02 1e+01))))

(fn GetDynamiteSpawnLocation
  (return (Transformation|GetWorldLocation (Variables|Default|GetDynamiteSpawnPoint))))