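; ShipShield is a shield Blueprint for a ship: a sphere mesh, hidden at start, that reacts to incoming hits.
; Shot and component hits broadcast OnReceiveShot and reveal the sphere.
; Component hits also pass the impact point to a dynamic material instance, where a timeline drives a radius parameter from that spot.
; Deactivate hides the sphere, disables its collision and broadcasts OnDeactivated.
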(event OnComponentHit(SphereMaterial)
  (params (HitComponent :type Primitive%20Component%20Object%20Reference) (OtherActor :type Actor%20Object%20Reference) (OtherComp :type Primitive%20Component%20Object%20Reference) (NormalImpulse :type Vector :default "0, 0, 0") (Hit :type Hit%20Result%20Structure%20%28by%20ref%29))
  (bind _spherematerial (Variables|Default|GetSphereMaterial))
  (Default|CallOnReceiveShot)
  (Rendering|SetVisibility _spherematerial true true)
  (bind _returnvalue (Rendering|Material|CreateDynamicMaterialInstance _spherematerial 0 0 :!class /Script/Engine.PrimitiveComponent))
  (Rendering|Material|SetVectorParameterValue _returnvalue "pos" (Math|Conversions|ToLinearColor(Vector) (.impactpoint Hit)) :!class /Script/Engine.MaterialInstanceDynamic)
  (bind _newtrack_0 (Timeline|animate PlayFromStart)
    (:Update
      (Rendering|Material|SetScalarParameterValue _returnvalue "radius" (* _newtrack_0 1.5e+02) :!class /Script/Engine.MaterialInstanceDynamic))))

(event Custom|Deactivate
  (bind _spherematerial (Variables|Default|GetSphereMaterial))
  (Rendering|SetVisibility _spherematerial false true)
  (Collision|SetCollisionEnabled _spherematerial "NoCollision")
  (Default|CallOnDeactivated))

(event EventShot
  (params (Hit :type Hit%20Result%20Structure))
  (Default|CallOnReceiveShot)
  (Rendering|SetVisibility (Variables|Default|GetSphereMaterial) true true))

(event EventBeginPlay
  (Rendering|SetVisibility (Variables|Default|GetSphereMaterial) false true))

(fn ConstructionScript)