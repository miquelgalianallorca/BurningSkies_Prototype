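; Mission trigger zone where the player plants dynamite by pressing Reload.
; While the zone is not hidden, player overlap toggles its input and the PressReload prompt.
; The first press spawns a DynamiteDropped actor just ahead of player character 0, then fires the OnExplosivesDropped dispatcher.
; A DoOnce limits the drop to a single use, though the prompt still follows overlap afterwards.
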(event Custom|DynamiteDropped
  (bind _returnvalue (Game|GetPlayerCharacter 0))
  (Utilities|FlowControl|DoOnce false
    (:Completed
      (Game|SpawnActorfromClass "/Game/Blueprints/Objects/DynamiteDropped.DynamiteDropped_C" (Math|Transform|MakeTransform (+ (Transformation|GetActorLocation _returnvalue) (* (Transformation|GetActorForwardVector _returnvalue) 1e+02)) "0, 0, 0" "1,1,1") "AlwaysSpawn" 0 0)
      (Default|CallOnExplosivesDropped))))

(event Collision|EventActorBeginOverlap
  (params (OtherActor :type Actor%20Object%20Reference))
  (if (not (Variables|Rendering|GetbHidden))
    (Development|PrintString "BeginOverlap")
    (Utilities|Casting|CastToPlayerCharacter OtherActor)
    (Input|EnableInput (Game|GetPlayerController 0))
    (Development|SetHiddeninGame (Variables|Default|GetPressReload) false false)))

(event EventBeginPlay
  (Development|SetHiddeninGame (Variables|Default|GetPressReload) true false))

(event Collision|EventActorEndOverlap
  (params (OtherActor :type Actor%20Object%20Reference))
  (if (not (Variables|Rendering|GetbHidden))
    (Development|PrintString "EndOverlap")
    (Utilities|Casting|CastToPlayerCharacter OtherActor)
    (Input|DisableInput (Game|GetPlayerController 0))
    (Development|SetHiddeninGame (Variables|Default|GetPressReload) true false)))

(event Input|ActionEvents|InputActionReload
  (params (Key :type Key%20Structure))
  (:Pressed
    (CallFunction|DynamiteDropped)))

(fn ConstructionScript)