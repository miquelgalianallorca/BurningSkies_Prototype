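; Airship destruction Blueprint for a mission, which fires explosion and fire effects and tracks whether the player is inside the airship area.
; The Explode event activates three explosion and three fire components together.
; Overlap begin and end on an inside-area trigger set and clear a player-in-trigger flag, with no check on which actor overlaps.
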(event OnComponentBeginOverlap(InsideAreaTrigger)
  (params (OverlappedComponent :type Primitive%20Component%20Object%20Reference) (OtherActor :type Actor%20Object%20Reference) (OtherComp :type Primitive%20Component%20Object%20Reference) (OtherBodyIndex :type Integer) (bFromSweep :type Boolean) (SweepResult :type Hit%20Result%20Structure%20%28by%20ref%29))
  (Variables|Default|SetIsPlayerInTrigger true))

(event OnComponentEndOverlap(InsideAreaTrigger)
  (params (OverlappedComponent :type Primitive%20Component%20Object%20Reference) (OtherActor :type Actor%20Object%20Reference) (OtherComp :type Primitive%20Component%20Object%20Reference) (OtherBodyIndex :type Integer))
  (Variables|Default|SetIsPlayerInTrigger false))

(event Custom|Explode
  (Components|Activation|Activate (Variables|Default|GetExplosion1) false))

(fn ConstructionScript)