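; Flying enemy character with a jetpack and an automatic weapon, which it spawns and attaches to its mesh on BeginPlay.
; Shot events subtract critical damage for head hits, hiding that bone, or normal damage otherwise, then play a hit-react montage.
; At zero life it stops flying, triggers a particle event, loses its controller, and drops as a physics body with its detached weapon before both are destroyed after a delay.
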(event OnComponentHit(CapsuleComponent)
  (params (HitComponent :type Primitive%20Component%20Object%20Reference) (OtherActor :type Actor%20Object%20Reference) (OtherComp :type Primitive%20Component%20Object%20Reference) (NormalImpulse :type Vector :default "0, 0, 0") (Hit :type Hit%20Result%20Structure%20%28by%20ref%29)))

(event EventBeginPlay
  (bind _asplayer_anim_bp (Utilities|Casting|CastToPlayerAnimBP (Components|SkeletalMesh|GetAnimInstance (Variables|Character|GetMesh))))
  (Default|SetFlying _asplayer_anim_bp true)
  (bind _returnvalue (Game|SpawnActorfromClass "/Game/Blueprints/Weapons/AutomaticWeapon.AutomaticWeapon_C" (Transformation|GetActorTransform) "Undefined" 0 0))
  (bind _output_get (Variables|Default|SetEnemyWeapon _returnvalue))
  (Transformation|AttachComponentToComponent _output_get (Variables|Character|GetMesh) "Weapon" "SnapToTarget" "KeepRelative" "KeepRelative" true))

(event Collision|EventActorBeginOverlap
  (params (OtherActor :type Actor%20Object%20Reference)))

(event EventTick
  (params (DeltaSeconds :type Float%20%28single-precision%29)))

(event EventShot
  (params (Hit :type Hit%20Result%20Structure))
  (bind (_bblockinghit _binitialoverlap _time _distance _location _impactpoint _normal _impactnormal _physmat _hitactor _hitcomponent _hitbonename) (Collision|BreakHitResult Hit))
  (bind _mesh (Variables|Character|GetMesh))
  (bind _enemyweapon (Variables|Default|GetEnemyWeapon))
  (bind _mesh_2 (Variables|Character|GetMesh))
  (bind _returnvalue (Components|SkeletalMesh|GetAnimInstance _mesh))
  (bind _returnvalue_2 (Actor|GetComponentbyClass _enemyweapon "/Script/Engine.SkeletalMeshComponent"))
  (bind _asskeletal_mesh_component (Utilities|Casting|CastToSkeletalMeshComponent _hitcomponent))
  (if (Utilities|Name|Equal(Name) _hitbonename "Head")
    (Variables|Default|SetLife (- (Variables|Default|GetLife) (Variables|Default|GetcriticalDamage)))
    (Components|SkinnedMesh|HideBonebyName _asskeletal_mesh_component _hitbonename "PBO_None")
    (else
      (Variables|Default|SetLife (- (Variables|Default|GetLife) (Variables|Default|GetnormalDamage)))))
  (bind _asplayer_anim_bp (Utilities|Casting|CastToPlayerAnimBP _returnvalue))
  (Animation|Montage|MontagePlay _returnvalue "/Game/Mannequin/Animations/Hit_React_1_Montage.Hit_React_1_Montage" 1.0 "MontageLength" 0.0)
  (if (<= (Variables|Default|GetLife) 0)
    (Default|SetFlying _asplayer_anim_bp false)
    (Class|ParticleSystemComponent|GenerateParticleEvent (Variables|Default|Getdead) "None" 0.0 "0, 0, 0" "0, 0, 0" "0, 0, 0")
    (Class|Pawn|DetachfromControllerPendingDestroy)
    (Physics|SetSimulatePhysics _mesh_2 true)
    (Collision|SetCollisionEnabled _mesh_2 "PhysicsOnly")
    (Transformation|DetachFromActor (Variables|Default|GetEnemyWeapon) "KeepWorld" "KeepWorld" "KeepWorld")
    (Utilities|IsValid _returnvalue_2
      (:Is%20Valid
        (Collision|SetCollisionEnabled _returnvalue_2 "PhysicsOnly")
        (Physics|SetSimulatePhysics _returnvalue_2 true)
        (Class|PrimitiveComponent|SetMassOverrideinKg (Variables|Character|GetMesh) "None" 4e+02 true)
        (Class|PrimitiveComponent|SetMassOverrideinKg _returnvalue_2 "None" 4e+02 true)
        (Utilities|FlowControl|Delay 5.0)
        (Actor|DestroyActor (Variables|Default|GetEnemyWeapon))
        (Actor|DestroyActor)))))

(fn ConstructionScript
  (Transformation|AttachComponentToComponent (Variables|Default|GetEnemyJetpack) (Variables|Character|GetMesh) "jetpack" "SnapToTarget" "SnapToTarget" "KeepWorld" true))