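; AI controller for the flying turret enemy that patrols waypoints and shoots at the player.
; While out of range, it gathers Waypoints listing its pawn, shuffles them and moves to the first, repeating after a delay when each move completes.
; Tick checks player distance; in range, it turns the pawn toward the player and fires its weapon, using Delay nodes to pace shots and pause for magazine refills.
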(event Custom|ReceiveMoveCompleted_Event_0
  (params (RequestID :type AI%20Request%20ID%20Structure) (Result :type EPathFollowingResult%20Enum :default "Success"))
  (bind _routes (Variables|Default|GetRoutes))
  (Utilities|FlowControl|Delay 3.0)
  (if (not (Variables|Default|GetisInRange))
    (bind _outactors (Actor|GetAllActorsOfClass "/Game/Blueprints/Enemy/WayPoint.Waypoint_C"))
    (bind _asenemy_flying_turrey (Utilities|Casting|CastToEnemyFlyingTurrey (Pawn|GetControlledPawn)))
    (for _array_element _outactors
      (if (!= (Utilities|Array|FindItem (Variables|/Game/Blueprints/Enemy/WayPoint.Waypoint_C|GetFlyingTurrets _array_element) _asenemy_flying_turrey) -1)
        (Utilities|Array|Add (Variables|Default|GetRoutes) _array_element)))
    (Utilities|Array|Shuffle _routes)
    (AI|Navigation|MovetoActor (Utilities|Array|Get(acopy) _routes) -1.0 true true)))

(event EventBeginPlay
  (bind _routes (Variables|Default|GetRoutes))
  (EventDispatchers|BindEventtoReceiveMoveCompleted (delegate Custom|ReceiveMoveCompleted_Event_0))
  (if (not (Variables|Default|GetisInRange))
    (bind _outactors (Actor|GetAllActorsOfClass "/Game/Blueprints/Enemy/WayPoint.Waypoint_C"))
    (bind _asenemy_flying_turrey (Utilities|Casting|CastToEnemyFlyingTurrey (Pawn|GetControlledPawn)))
    (for _array_element _outactors
      (if (!= (Utilities|Array|FindItem (Variables|/Game/Blueprints/Enemy/WayPoint.Waypoint_C|GetFlyingTurrets _array_element) _asenemy_flying_turrey) -1)
        (Utilities|Array|Add (Variables|Default|GetRoutes) _array_element)))
    (Utilities|Array|Shuffle _routes)
    (AI|Navigation|MovetoActor (Utilities|Array|Get(acopy) _routes) -1.0 true true)))

(event EventTick
  (params (DeltaSeconds :type Float%20%28single-precision%29))
  (bind _returnvalue (Pawn|GetControlledPawn))
  (bind _returnvalue_2 (Game|GetPlayerCharacter 0))
  (bind _returnvalue_3 (Pawn|GetControlledPawn))
  (if (Variables|Default|GetisInRange)
    (Transformation|SetActorRotation _returnvalue_3 (Math|Rotator|FindLookatRotation (Transformation|GetActorLocation _returnvalue_3) (Transformation|GetActorLocation _returnvalue_2))))
  (if (<= (Transformation|GetDistanceTo _returnvalue_3 _returnvalue_2) 1.5e+03)
    (Variables|Default|SetisInRange true)
    (bind _asenemy_flying_turrey (Utilities|Casting|CastToEnemyFlyingTurrey _returnvalue))
    (Utilities|FlowControl|Delay 0.4)
    (if (> (Variables|Default|GetBullets) 0)
      (Variables|Default|SetBullets (- (Variables|Default|GetBullets) 1))
      (else
        (Variables|Default|SetBullets (Variables|Default|GetNumBullets))
        (Utilities|FlowControl|Delay 2.0)))
    (Class|Weapon|EnemyShoot(Message) (Variables|/Game/Blueprints/Enemy/EnemyFlyingTurrey.EnemyFlyingTurrey_C|GetEnemyWeapon _asenemy_flying_turrey) (Game|GetPlayerCharacter 0) _returnvalue)
    (else
      (Variables|Default|SetisInRange false))))

(fn ConstructionScript)