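; EnemyTarget is a turret-style enemy that detects the player within range, turns to face them and fires bullets until shot.
; Each Tick while alive, a sphere overlap at the Arrow finds PlayerCharacter pawns and rotates the actor toward the first.
; Detection changes start or clear a looping Fire timer and swap the cylinder between red and yellow.
; A Shot event kills it permanently, stopping fire and turning it green.
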(event EventTick
  (params (DeltaSeconds :type Float%20%28single-precision%29))
  (bind _playerdetected (Variables|Combat|GetplayerDetected))
  (if (not (Variables|Default|GetisDead))
    (bind _detected (CallFunction|DetectPlayer))
    ;[1 1 1] Enable/Disable Shooting
    (if _detected
      (if (not _playerdetected)
        (Combat|AggroStart))
      (elif _playerdetected
        (Combat|AggroEnd)))))

(event EventShot
  (params (Hit :type Hit%20Result%20Structure))
  ;[1 1 1] Receive Shot
  (if (not (Variables|Default|GetisDead))
    (CallFunction|Kill)))

(fn ConstructionScript)

(fn Fire
  (Game|SpawnActorfromClass "/Game/Blueprints/Characters/Bullet.Bullet_C" (Math|Transform|MakeTransform (Transformation|GetWorldLocation (Variables|Default|GetArrow)) (Math|Conversions|RotationFromXVector (Transformation|GetActorForwardVector))) "Undefined" 0 self)
  (return))

(fn Kill
  (Variables|Default|SetisDead true)
  (Rendering|Material|SetMaterial (Variables|Default|GetCylinder) 0 "/Game/Blueprints/Materials/GreenMat.GreenMat")
  (Utilities|Time|ClearTimerbyFunctionName self "Fire")
  (return))

(fn DetectPlayer
  (bind _outactors (Collision|SphereOverlapActors (Transformation|GetWorldLocation (Variables|Default|GetArrow)) (Variables|Combat|GetdetectRange) (Utilities|Array|MakeArray "ObjectTypeQuery3") "/Game/Blueprints/Characters/PlayerCharacter.PlayerCharacter_C"))
  (bind _array_element (Utilities|Array|ForEachLoopwithBreak _outactors)
    (:LoopBody
      ;[1 1 1] Face Player
      (Transformation|SetActorRotation (Math|Rotator|FindLookatRotation (Transformation|GetActorLocation) (Transformation|GetActorLocation _array_element)))
      (return true))
    (:Completed
      (return false))))

(fn AggroStart
  (Variables|Combat|SetplayerDetected true)
  (Utilities|Time|SetTimerbyFunctionName self "Fire" (Variables|Combat|GetfireRate) true)
  (Rendering|Material|SetMaterial (Variables|Default|GetCylinder) 0 "/Game/Blueprints/Materials/RedMat.RedMat")
  (return))

(fn AggroEnd
  (Variables|Combat|SetplayerDetected false)
  (Utilities|Time|ClearTimerbyFunctionName self "Fire")
  (Rendering|Material|SetMaterial (Variables|Default|GetCylinder) 0 "/Game/Blueprints/Materials/YellowMat.YellowMat")
  (return))