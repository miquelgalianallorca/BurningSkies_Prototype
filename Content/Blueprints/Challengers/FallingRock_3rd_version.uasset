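; A falling rock hazard that drops under physics and damages the player on impact.
; A player entering its trigger zone starts the fall after a delay, while a Shot event or a hit involving a rocket or another rock starts it immediately.
; Tick enables mesh physics once falling, with linear damping set at BeginPlay as air friction.
; While armed, hitting the player reduces HealthComp life, plays an explosion sound and disarms the rock.
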(event OnActorBeginOverlap(ZonaDeTrigger)
  (params (OverlappedActor :type Actor%20Object%20Reference) (OtherActor :type Actor%20Object%20Reference))
  (Utilities|Casting|CastToPlayerCharacter OtherActor)
  (Utilities|FlowControl|Delay (Variables|Default|GetDelayDeCaidaxTrigger))
  (Variables|Default|SetFallDown true)
  (Variables|Default|SetCanHurtPlayer true))

(event EventBeginPlay
  (Class|PrimitiveComponent|SetLinearDamping (Variables|Default|GetStaticMesh) (Variables|Default|GetFriccionDelAire)))

(event Collision|EventHit
  (params (MyComp :type Primitive%20Component%20Object%20Reference) (Other :type Actor%20Object%20Reference) (OtherComp :type Primitive%20Component%20Object%20Reference) (bSelfMoved :type Boolean) (HitLocation :type Vector :default "0, 0, 0") (HitNormal :type Vector :default "0, 0, 0") (NormalImpulse :type Vector :default "0, 0, 0") (Hit :type Hit%20Result%20Structure%20%28by%20ref%29))
  (Utilities|FlowControl|Sequence
    (:then_0
      (if (Variables|Default|GetCanHurtPlayer)
        (bind _asplayer_character (Utilities|Casting|CastToPlayerCharacter Other))
        (Variables|/Game/Blueprints/Characters/HealthComp.HealthComp_C|SetcurrentLife (Actor|GetComponentbyClass _asplayer_character "/Game/Blueprints/Characters/HealthComp.HealthComp_C") (- (Variables|/Game/Blueprints/Characters/HealthComp.HealthComp_C|GetcurrentLife (Actor|GetComponentbyClass _asplayer_character "/Game/Blueprints/Characters/HealthComp.HealthComp_C")) 2e+01))
        (Audio|PlaySoundatLocation "/Game/Audio/Explosion.Explosion" "0, 0, 0" "0, 0, 0" 0.1)
        (Variables|Default|SetCanHurtPlayer false)))
    (:then_1
      (Utilities|Casting|CastToFallingRock_3rd_version Other)
      (Variables|Default|SetFallDown true :!label _label)
      (Variables|Default|SetCanHurtPlayer true))
    (:then_3
      (Utilities|Casting|CastToRocketProjectile Other)
      (goto _label))))

(event EventTick
  (params (DeltaSeconds :type Float%20%28single-precision%29))
  (if (Variables|Default|GetFallDown)
    (Physics|SetSimulatePhysics (Variables|Default|GetStaticMesh) true)))

(event EventShot
  (params (Hit :type Hit%20Result%20Structure) (FromFlamethrower :type Boolean))
  (Variables|Default|SetFallDown true)
  (Variables|Default|SetCanHurtPlayer true))

(fn ConstructionScript)