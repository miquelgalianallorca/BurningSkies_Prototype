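; Ring checkpoint for the "Rings" challenge, counted only when the player character crosses it in sequence, optionally gated by the controller's time flag.
; On overlap, it checks its Id against the shared ControllerGeneral counter, advances it, resets its arch material and turns the next arch gold.
; Brief RetoIsla widgets show progress.
; The final ring shows a completion message, then destroys all waypoints and the controller.
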(event Collision|EventActorBeginOverlap
  (params (OtherActor :type Actor%20Object%20Reference))
  (bind _returnvalue (Game|GetPlayerController 0))
  (bind _controller_general (Variables|Default|GetController_General))
  (bind _controller_general_2 (Variables|Default|GetController_General))
  (bind _controller_general_3 (Variables|Default|GetController_General))
  (bind _id (Variables|Default|GetId))
  (bind _id_2 (Variables|Default|GetId))
  (bind _waypoints (Variables|/Game/Blueprints/Challengers/Reto_Controllador_General.Reto_Controllador_General_C|GetWaypoints _controller_general))
  (bind _returnvalue_2 (Utilities|Array|Length _waypoints))
  (bind _returnvalue_3 (== _id _returnvalue_2))
  (Utilities|Casting|CastToPlayerCharacter OtherActor)
  (if (Variables|/Game/Blueprints/Challengers/Reto_Controllador_General.Reto_Controllador_General_C|GetAct/Des_Tiempo _controller_general)
    (if (Variables|/Game/Blueprints/Challengers/Reto_Controllador_General.Reto_Controllador_General_C|GetTiempo _controller_general)
      (for _index (range 1 _returnvalue_2) :!label _label
        (if (== (- (Variables|Default|GetId) 1) (Variables|/Game/Blueprints/Challengers/Reto_Controllador_General.Reto_Controllador_General_C|GetSuma _controller_general_2))
          (Variables|/Game/Blueprints/Challengers/Reto_Controllador_General.Reto_Controllador_General_C|SetSuma _controller_general_2 _id_2)
          (Rendering|Material|SetMaterial (Variables|/Script/Engine.StaticMeshActor|GetStaticMeshComponent (Variables|Default|Getarco)) 0 "/Game/FirstPerson/Meshes/BaseMaterial.BaseMaterial")
          (if _returnvalue_3
            _
            (else
              (Rendering|Material|SetMaterial (Variables|/Script/Engine.StaticMeshActor|GetStaticMeshComponent (Variables|Default|GetarcoSiguiente)) 0 "/Game/Material/MI_emissivegold.MI_emissivegold")))
          (bind _returnvalue_4 (UserInterface|CreateWidget "/Game/Blueprints/UI/RetoIsla.RetoIsla_C" _returnvalue))
          (if (== _id_2 1)
            (Default|MeterTexto _returnvalue_4 "Cross all the rings. Crossed 1 ")
            (UserInterface|Viewport|AddtoPlayerScreen _returnvalue_4)
            (Utilities|FlowControl|Delay 1.3)
            (else
              (Default|MeterTexto _returnvalue_4 (Utilities|String|ToString(Integer) _id_2))
              (UserInterface|Viewport|AddtoPlayerScreen _returnvalue_4)
              (Utilities|FlowControl|Delay 0.5)))
          (Widget|RemovefromParent _returnvalue_4)))
      (if (== (Variables|/Game/Blueprints/Challengers/Reto_Controllador_General.Reto_Controllador_General_C|GetSuma _controller_general) _returnvalue_2)
        (if _returnvalue_3
          (Utilities|FlowControl|Delay 1.0)
          (bind _returnvalue_5 (UserInterface|CreateWidget "/Game/Blueprints/UI/RetoIsla.RetoIsla_C" _returnvalue))
          (Default|MeterTexto _returnvalue_5 "You completed the \"Rings\" challenge")
          (UserInterface|Viewport|AddtoPlayerScreen _returnvalue_5)
          (Utilities|FlowControl|Delay 2.0)
          (Widget|RemovefromParent _returnvalue_5)
          (Actor|DestroyActor (Variables|/Game/Blueprints/Challengers/Reto_Controllador_General.Reto_Controllador_General_C|GetWaypoints _controller_general_3))
          (Actor|DestroyActor _controller_general_3))))
    (else
      (goto _label))))

(fn ConstructionScript)

(fn NewFunction0)