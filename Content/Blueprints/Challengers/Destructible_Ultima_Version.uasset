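; Destructible challenger actor that shatters on impact and plays a quiet, one-time explosion sound on player contact once armed.
; Component hits from rocket projectiles always apply massive damage, while falling rocks and other instances of this class do so only when their flags allow it.
; Breaking, or the Shot event, arms the sound flag, so the sound waits for a later player hit rather than playing on destruction.
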(event OnComponentHit(Destructible)
  (params (HitComponent :type Primitive%20Component%20Object%20Reference) (OtherActor :type Actor%20Object%20Reference) (OtherComp :type Primitive%20Component%20Object%20Reference) (NormalImpulse :type Vector :default "0, 0, 0") (Hit :type Hit%20Result%20Structure%20%28by%20ref%29))
  (bind _impactpoint (Collision|BreakHitResult Hit))
  (Utilities|FlowControl|Sequence
    (:then_0
      (Utilities|Casting|CastToPlayerCharacter OtherActor)
      (if (Variables|Default|GetSuenaAlContacto?)
        (if (not (Variables|Default|GetHasPlayed))
          (Audio|PlaySoundatLocation "/Game/Audio/Explosion.Explosion" "0, 0, 0" "0, 0, 0" 0.1)
          (Variables|Default|SetHasPlayed true))))
    (:then_1
      (if (Variables|Default|GetLeAfectanRocasCaidas?)
        (Utilities|Casting|CastToFallingRock_3rd_version OtherActor)
        (Class|DestructibleComponent|ApplyDamage (Variables|Default|GetDestructible) 1e+10 _impactpoint _impactpoint 1e+03 :!label _label)
        (Variables|Default|SetSuenaAlContacto? true)))
    (:then_2
      (if (Variables|Default|GetLeAfectanDestructibles?)
        (Utilities|Casting|CastToDestructible_Ultima_Version OtherActor)
        (goto _label)))
    (:then_3
      (Utilities|Casting|CastToRocketProjectile OtherActor)
      (goto _label))))

(event EventBeginPlay)

(event Collision|EventActorBeginOverlap
  (params (OtherActor :type Actor%20Object%20Reference)))

(event EventShot
  (params (Hit :type Hit%20Result%20Structure) (FromFlamethrower :type Boolean) (OriginLocation :type Vector :default "0, 0, 0"))
  (Variables|Default|SetSuenaAlContacto? true))

(fn ConstructionScript)