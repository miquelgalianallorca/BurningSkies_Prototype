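; Reto_1 is a checkpoint trigger for an ordered three-step challenge, activated when the PlayerCharacter overlaps it.
; Its Id selects which Comprobación flag it sets on the Reto_1_General actor held in Controller, with steps 2 and 3 requiring the previous flag.
; Completed steps 1 and 2 destroy their trigger, while step 3 prints a congratulations message and destroys the Controller instead.
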(event EventBeginPlay)

(event Collision|EventActorBeginOverlap
  (params (OtherActor :type Actor%20Object%20Reference))
  (bind _controller (Variables|Default|GetController))
  (Utilities|Casting|CastToPlayerCharacter OtherActor)
  (if (== (Variables|Default|GetId) 1)
    (bind _asreto_1_general (Utilities|Casting|CastToReto_1_General _controller))
    (Variables|/Game/Blueprints/Challengers/Reto_1_General.Reto_1_General_C|SetComprobación_1 _asreto_1_general true)
    (Actor|DestroyActor)
    (elif (== (Variables|Default|GetId) 2)
      (bind _asreto_1_general_2 (Utilities|Casting|CastToReto_1_General _controller))
      (if (Variables|/Game/Blueprints/Challengers/Reto_1_General.Reto_1_General_C|GetComprobación_1 _asreto_1_general_2)
        (Variables|/Game/Blueprints/Challengers/Reto_1_General.Reto_1_General_C|SetComprobación_2 _asreto_1_general_2 true)
        (Actor|DestroyActor))
      (elif (== (Variables|Default|GetId) 3)
        (bind _asreto_1_general_3 (Utilities|Casting|CastToReto_1_General _controller))
        (if (Variables|/Game/Blueprints/Challengers/Reto_1_General.Reto_1_General_C|GetComprobación_2 _asreto_1_general_3)
          (Variables|/Game/Blueprints/Challengers/Reto_1_General.Reto_1_General_C|SetComprobación_3 _asreto_1_general_3 true)
          (Development|PrintString "Enhorabuena!!")
          (Actor|DestroyActor (Variables|Default|GetController)))))))

(fn ConstructionScript)