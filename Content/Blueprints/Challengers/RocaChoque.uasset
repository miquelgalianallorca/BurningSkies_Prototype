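; RocaChoque is a component that makes its owning actor, likely a rock obstacle, knock the player back on collision.
; On a hit it activates the player's CharacterMovement and launches the character hard opposite the follow camera's forward vector.
; A short timer then deactivates movement again and sets the player anim Blueprint back to flying.
; An alternative knockback along the hit normal is left unconnected.
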(event Custom|OnActorHit_Event_0
  (params (SelfActor :type Actor%20Object%20Reference) (OtherActor :type Actor%20Object%20Reference) (NormalImpulse :type Vector) (Hit :type Hit%20Result%20Structure%20%28by%20ref%29))
  (bind _asplayer_character (Utilities|Casting|CastToPlayerCharacter OtherActor))
  (Components|Activation|Activate (Actor|GetComponentbyClass _asplayer_character "/Script/Engine.CharacterMovementComponent") false)
  (Character|LaunchCharacter _asplayer_character (* (Math|Vector|GetForwardVector (Variables|/Game/Blueprints/Characters/PlayerCharacter.PlayerCharacter_C|GetFollowCamera _asplayer_character)) -2e+04) true true)
  (Variables|Default|SetMoveComp (Actor|GetComponentbyClass _asplayer_character "/Script/Engine.CharacterMovementComponent"))
  (Utilities|Time|SetTimerbyEvent (delegate Custom|DeactivateCharacterMovement) 0.1))

(event Custom|DeactivateCharacterMovement
  (Components|Activation|Deactivate (Actor|GetComponentbyClass (stale Custom|OnActorHit_Event_0 _asplayer_character) "/Script/Engine.CharacterMovementComponent"))
  (bind _asplayer_anim_bp (Utilities|Casting|CastToPlayerAnimBP (Components|SkeletalMesh|GetAnimInstance (Variables|/Script/Engine.Character|GetMesh (stale Custom|OnActorHit_Event_0 _asplayer_character)))))
  (Variables|/Game/Mannequin/Animations/PlayerAnimBP.PlayerAnimBP_C|SetIsInAir? _asplayer_anim_bp false)
  (Variables|/Game/Mannequin/Animations/PlayerAnimBP.PlayerAnimBP_C|SetisFlying? _asplayer_anim_bp true))

(event EventBeginPlay
  (Collision|AssignOnActorHit (Components|GetOwner) (delegate Custom|OnActorHit_Event_0)))