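; General challenge controller actor that runs a time limit for a challenge the player starts by overlapping it.
; BeginPlay converts the minutes and seconds variables into a total in seconds.
; A player overlap, gated by ActDesTiempo and EmpFinalTempo, sets Tiempo and starts a one-shot timer.
; On expiry, Activar_Tiempo clears Tiempo, prints a failure message and re-arms EmpFinalTempo for another attempt; no success handling is present here.
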(event Custom|Activar_Tiempo
  (Variables|Default|SetTiempo false)
  (Development|PrintString "RETO FALLIDO, VUELVE A COGER EL RETO")
  (Variables|Default|SetEmp/Final%20tempo true))

(event EventBeginPlay
  (Variables|Default|SetTiempoTotalDelReto (+ (* (Variables|Default|GetMinutos_Publica) 6e+01) (Variables|Default|GetSegundos_Publica))))

(event Collision|EventActorBeginOverlap
  (params (OtherActor :type Actor%20Object%20Reference))
  (Utilities|Casting|CastToPlayerCharacter OtherActor)
  (if (Variables|Default|GetAct/Des_Tiempo)
    (if (Variables|Default|GetEmp/Final%20tempo)
      (Development|PrintString "Tiempo empezado")
      (Variables|Default|SetTiempo true)
      (Utilities|Time|SetTimerbyEvent (delegate Custom|Activar_Tiempo) (Variables|Default|GetTiempoTotalDelReto))
      (Variables|Default|SetEmp/Final%20tempo false))))

(fn ConstructionScript)