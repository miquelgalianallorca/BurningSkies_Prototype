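; Rocket launcher weapon Blueprint that fires homing rocket projectiles toward the player camera's aim point, with loader and backup ammo.
; Shoot fires once per press via a DoOnce reset on release, gated by a rate-of-fire cooldown timer.
; It spawns the rocket at the muzzle rotated toward a point at Range along the camera forward, then triggers homing and sets damage.
; An empty loader triggers Reload, which refills from backup ammo and prints counts.
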(event Custom|CoolDown
  (Variables|Default|SetisReadyToFire true))

(event EventReleaseShoot
  (bind _returnvalue (Game|GetPlayerCharacter 0))
  (bind _projectilespawnpoint (Variables|Default|GetProjectileSpawnPoint))
  (bind _returnvalue_2 (Transformation|GetWorldLocation _projectilespawnpoint))
  (bind _returnvalue_3 (Actor|GetComponentbyClass _returnvalue "/Script/Engine.CameraComponent"))
  (Utilities|FlowControl|DoOnce false) ; enters at Reset
)

(event EventReload
  ;[1 1 1] Reload weapon
  (if (and (> (Variables|Default|GetBackupCurrentCapacity) 0) (> (Variables|Default|GetLoaderMaxCapacity) (Variables|Default|GetLoaderCurrentCapacity)))
    (bind _output_get (Variables|Default|SetAmmoToReload (Math|Integer|Min(Integer) (Variables|Default|GetBackupCurrentCapacity) (- (Variables|Default|GetLoaderMaxCapacity) (Variables|Default|GetLoaderCurrentCapacity)))))
    (Variables|Default|SetLoaderCurrentCapacity (+ _output_get (Variables|Default|GetLoaderCurrentCapacity)))
    (Variables|Default|SetBackupCurrentCapacity (- (Variables|Default|GetBackupCurrentCapacity) _output_get))
    (Development|PrintString (Utilities|String|Append "- RELOAD - 
Current ammo: " (Utilities|String|ToString(Integer) (Variables|Default|GetLoaderCurrentCapacity)) " 
Backup ammo: " (Utilities|String|ToString(Integer) (Variables|Default|GetBackupCurrentCapacity))) true true "(R=0.250000,G=0.000000,B=1.000000,A=1.000000)" 5.0)))

(event EventShoot
  (params (isZooming :type Boolean))
  (bind _returnvalue (Game|GetPlayerCharacter 0))
  (bind _projectilespawnpoint (Variables|Default|GetProjectileSpawnPoint))
  (bind _returnvalue_2 (Transformation|GetWorldLocation _projectilespawnpoint))
  (bind _returnvalue_3 (Actor|GetComponentbyClass _returnvalue "/Script/Engine.CameraComponent"))
  (if (Variables|Default|GetisReadyToFire)
    (if (> (Variables|Default|GetLoaderCurrentCapacity) 0)
      (Utilities|FlowControl|DoOnce false
        (:Completed
          (Variables|Default|SetisReadyToFire false)
          (Utilities|Time|SetTimerbyEvent (delegate Custom|CoolDown) (Variables|Default|GetRateOfFire))
          (bind _returnvalue_4 (Game|SpawnActorfromClass "/Game/Blueprints/Weapons/RocketProjectile.RocketProjectile_C" (Math|Transform|MakeTransform _returnvalue_2 (Math|Rotator|MakeRotfromX (- (+ (* (Math|Vector|GetForwardVector _returnvalue_3) (Variables|Default|GetRange)) (Transformation|GetWorldLocation _returnvalue_3)) _returnvalue_2))) "Undefined" 0 0))
          (Default|HomingMissile _returnvalue_4)
          (Variables|/Game/Blueprints/Weapons/RocketProjectile.RocketProjectile_C|SetDamage _returnvalue_4 (Variables|Default|GetDamage))
          (Math|Integer|DecrementInt (Variables|Default|GetLoaderCurrentCapacity))))
      (else
        (CallFunction|Reload)))))

(event EventBeginPlay
  ;[1 1 1] Init weapon
  (|CallParentFunction)
  (Variables|Default|SetLoaderCurrentCapacity (Variables|Default|GetLoaderMaxCapacity))
  (Variables|Default|SetBackupCurrentCapacity (Variables|Default|GetBackupMaxCapacity)))

(fn ConstructionScript
  (|CallParentFunction))