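; Automatic gun weapon Blueprint that fires hitscan shots on a looping timer while shooting is held, with an automatic reload when the magazine empties.
; Each shot plays camera shake, sound and muzzle flash, then traces from the player camera, adding random spread unless aiming.
; Hits send a shot message, apply radial damage and spawn decal and impact particles; every shot spawns a bullet trail from the muzzle.
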(event Custom|ShootFX
  ;[1 1 1] ShootFX - MuzzleFlash + Sound
  (Audio|SpawnSoundatLocation "/Game/Audio/shootSFX.shootSFX" (Transformation|GetWorldLocation (Variables|Default|GetProjectileSpawnPoint)))
  (Components|Activation|Activate (Variables|Default|GetParticleSystem) false)
  (Utilities|FlowControl|Delay 0.1)
  (Components|Activation|Deactivate (Variables|Default|GetParticleSystem)))

(event Custom|Fire
  (bind _returnvalue (Game|GetPlayerCharacter 0))
  ;[1 1 1] Fire
  (if (and (> (Variables|Default|GetLoaderCurrentCapacity) 0) (Variables|Default|GetisReadyToFire))
    (Math|Integer|DecrementInt (Variables|Default|GetLoaderCurrentCapacity)
      (:%20%20
        (if (Variables|Default|GetisAiming)
          (Variables|AimOffset|SetShake%20Class "/Game/Blueprints/Weapons/CameraShakes/AutomaticGun_Shake_AIM.AutomaticGun_Shake_AIM_C")
          (else
            (Variables|AimOffset|SetShake%20Class "/Game/Blueprints/Weapons/CameraShakes/AutomaticGun_Shake.AutomaticGun_Shake_C")))
        (if (Utilities|IsValid _returnvalue)
          (Camera|PlayWorldCameraShake (Variables|AimOffset|GetShake%20Class) (Transformation|GetActorLocation _returnvalue) 0.0 5e+02))
        (CallFunction|ShootFX)
        (Utilities|FlowControl|Delay (Variables|Default|GetshootDelay))
        (CallFunction|RaycastNoAssist)))
    (else
      (Utilities|FlowControl|DoOnce false
        (:Completed
          (CallFunction|Reload))))))

(event EventReleaseShoot
  ;[1 1 1] Shoot/Release shoot event
  (Utilities|Time|ClearandInvalidateTimerbyHandle (Variables|Default|GetfireTimerHandle))
  (Utilities|FlowControl|DoOnce false) ; enters at Reset
)

(event EventShoot
  (params (isZooming :type Boolean))
  ;[1 1 1] Shoot/Release shoot event
  (Variables|Default|SetisAiming isZooming)
  (Utilities|FlowControl|DoOnce false
    (:Completed
      (CallFunction|Fire)
      (bind _returnvalue (Utilities|Time|SetTimerbyEvent (delegate Custom|Fire) (Variables|Default|GetRateOfFire) true))
      (Variables|Default|SetfireTimerHandle _returnvalue))))

(event EventShootBP
  (params (IsZooming :type Boolean))
  ;[1 1 1] Shoot/Release shoot event
  (Variables|Default|SetisAiming IsZooming))

(event EventReleaseShootBP
  ;[1 1 1] Shoot/Release shoot event
)

(event EventDeactivateWeapon
  ;[1 1 1] Change weapon
  (CallFunction|ReleaseShoot)
  (Rendering|SetVisibility (Variables|Default|GetAutomaticGunMesh) false true))

(event EventReload
  ;[1 1 1] Reload
  (Variables|Default|SetisReadyToFire false)
  (|CallParentFunction)
  (Utilities|FlowControl|Delay (Variables|Default|GetReloadTime))
  (Variables|Default|SetisReadyToFire true)
  (Development|PrintString (Utilities|String|Append "- RELOAD - 
Current ammo: " (Utilities|String|ToString(Integer) (Variables|Default|GetLoaderCurrentCapacity)) " 
Backup ammo: " (Utilities|String|ToString(Integer) (Variables|Default|GetBackupCurrentCapacity))) true true "(R=0.250000,G=0.000000,B=1.000000,A=1.000000)" 5.0)
  ;[1 1 1] Fire
  (Utilities|FlowControl|DoOnce false) ; enters at Reset
)

(event EventBeginPlay
  ;[1 1 1] Init weapon
  (|CallParentFunction)
  (Variables|Default|SetLoaderCurrentCapacity (Variables|Default|GetLoaderMaxCapacity))
  (Variables|Default|SetBackupCurrentCapacity (Variables|Default|GetBackupMaxCapacity)))

(event EventStopShooting
  ;[1 1 1] Stop shooting
  (Utilities|Time|ClearandInvalidateTimerbyHandle (Variables|Default|GetfireTimerHandle)))

(event EventActivateWeapon
  ;[1 1 1] Change weapon
  (CallFunction|ReleaseShoot)
  (Rendering|SetVisibility (Variables|Default|GetAutomaticGunMesh) true true))

(fn ConstructionScript)

(fn DrawDebugRay
  (params (startPos :type Vector) (endPos :type Vector))
  (Game|SpawnActorfromClass "/Game/Blueprints/Weapons/BulletTrail.BulletTrail_C" (Math|Transform|MakeTransform startPos (Math|Rotator|FindLookatRotation startPos endPos) "1,1,1") "AdjustIfPossibleButDontSpawnIfColliding" (Game|GetPlayerCharacter 0) 0)
  ;[1 1 1] Draw debug ray
  (if (Variables|Default|GetdrawDebugRays)
    (Collision|LineTraceByChannel startPos endPos "TraceTypeQuery2" false (Utilities|Array|MakeArray (Game|GetPlayerCharacter 0)) "ForDuration")))

(fn DrawFX
  (params (location :type Vector) (rotation :type Rotator))
  (Rendering|Decal|SpawnDecalatLocation "/Game/Material/M_Decal_BulletMark.M_Decal_BulletMark" "25.000000,25.000000,25.000000" location rotation 5.0)
  (Effects|SpawnEmitteratLocation "/Game/Effects/P_BulletImpact.P_BulletImpact" location rotation))

(fn GetRaycastBounds
  (bind _returnvalue (Game|GetPlayerCharacter 0))
  (bind _returnvalue_2 (Actor|GetComponentbyClass _returnvalue "/Script/Engine.CameraComponent"))
  (bind _returnvalue_3 (Actor|GetComponentbyClass _returnvalue "/Script/Engine.SpringArmComponent"))
  (bind _returnvalue_4 (Transformation|GetWorldLocation _returnvalue_2))
  (bind _returnvalue_5 (Math|Vector|GetForwardVector _returnvalue_2))
  (bind _targetarmlength (Variables|/Script/Engine.SpringArmComponent|GetTargetArmLength _returnvalue_3))
  (bind _returnvalue_6 (* _returnvalue_5 _targetarmlength))
  (bind _returnvalue_7 (+ _returnvalue_4 _returnvalue_6))
  (return _returnvalue_7 (+ _returnvalue_7 (* _returnvalue_6 (Variables|Default|GetMaxRange)))))

(fn GetBulletDeviation
  (bind _max_offset (Variables|AimOffset|GetMax%20Offset))
  (bind _min_offset (Variables|AimOffset|GetMin%20Offset))
  (bind _offset_index (Variables|AimOffset|GetOffset%20Index))
  (return (Math|Vector|MakeVector (* (Math|Random|RandomFloatinRange _min_offset _max_offset) _offset_index) (* (Math|Random|RandomFloatinRange _min_offset _max_offset) _offset_index) (* (Math|Random|RandomFloatinRange _min_offset _max_offset) _offset_index))))

(fn RaycastNoAssist
  (bind (_beginlocation _endlocation) (CallFunction|GetRaycastBounds))
  (if (Variables|Default|GetisAiming)
    (Variables|AimOffset|SetOffset%20Index 0.0)
    (else
      (Variables|AimOffset|SetOffset%20Index 1.0)))
  (bind (_outhit _returnvalue) (Collision|LineTraceByChannel _beginlocation (+ _endlocation (CallFunction|GetBulletDeviation)) "TraceTypeQuery1" false (Utilities|Array|MakeArray (Game|GetPlayerCharacter 0)) "None"))
  (if _returnvalue
    ;[1 1 1] Impact
    (Class|IShootable|ReceiveShot(Message) (.HitActor (Collision|BreakHitResult _outhit)) _outhit false)
    (Game|Damage|ApplyRadialDamage (Variables|Default|Getdamage_0) (.ImpactPoint (Collision|BreakHitResult _outhit)) (Variables|Default|GetdamageRadius) 0 0 (Game|GetPlayerCharacter 0) 0 false "ECC_Visibility")
    (CallFunction|DrawDebugRay (Transformation|GetWorldLocation (Variables|Default|GetProjectileSpawnPoint)) (.ImpactPoint (Collision|BreakHitResult _outhit)))
    (CallFunction|DrawFX (.ImpactPoint (Collision|BreakHitResult _outhit)) (Math|Conversions|RotationFromXVector (.ImpactNormal (Collision|BreakHitResult _outhit))))
    (else
      ;[1 1 1] Shooting at air
      (CallFunction|DrawDebugRay (Transformation|GetWorldLocation (Variables|Default|GetProjectileSpawnPoint)) _endlocation))))