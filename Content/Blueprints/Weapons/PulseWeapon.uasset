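; PulseWeapon is a chargeable gun Blueprint that can be shown or hidden on activation and deactivation.
; Shoot shows the charge effect and starts a Tick-driven timer capped near TimeToCharge.
; ReleaseShoot swaps to the fire material, calls Fire, then hides the effect after a short delay.
; Fire runs a debug-drawn line trace along the player camera's aim, with charge-scaled reach; its hit result is unused.
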(event Custom|Fire
  (bind _returnvalue (Game|GetPlayerCharacter 0))
  (bind _returnvalue_2 (Actor|GetComponentbyClass _returnvalue "/Script/Engine.CameraComponent"))
  (Collision|LineTraceByChannel (Transformation|GetWorldLocation (Variables|Default|GetRaycastSpawnPoint)) (+ (* (Math|Vector|GetForwardVector _returnvalue_2) (* (Variables|Default|GetWeaponCharge) (Variables|Default|GetdistanceToRay))) (Transformation|GetWorldLocation _returnvalue_2)) "TraceTypeQuery1" false 0 "ForDuration" true "(R=1.000000,G=0.000000,B=0.000000,A=1.000000)" "(R=0.000000,G=1.000000,B=0.000000,A=1.000000)" 2.0))

(event EventBeginPlay)

(event Collision|EventActorBeginOverlap
  (params (OtherActor :type Actor%20Object%20Reference)))

(event EventDeactivateWeapon
  (Rendering|SetVisibility (Variables|Default|GetPulseGunMesh) false true))

(event EventTick
  (params (DeltaSeconds :type Float%20%28single-precision%29))
  (if (Variables|Default|GetchargeWeapon)
    (if (<= (Variables|Default|GetWeaponCharge) (Math|Conversions|ToFloat(Integer) (Variables|Default|GetTimeToCharge)))
      (Variables|Default|SetWeaponCharge (+ (Variables|Default|GetWeaponCharge) DeltaSeconds)))))

(event EventReleaseShoot
  (bind _effect (Variables|Default|GetEffect))
  (Rendering|Material|SetMaterial (Variables|Default|GetEffect) 0 "/Game/Material/Fire.Fire")
  (CallFunction|Fire)
  (Utilities|FlowControl|Delay 0.5)
  (Rendering|Material|SetMaterial _effect 0 0)
  (Rendering|SetVisibility _effect false true)
  (Variables|Default|SetchargeWeapon false))

(event EventShoot
  (bind _effect (Variables|Default|GetEffect))
  (Variables|Default|SetchargeWeapon true)
  (Variables|Default|SetWeaponCharge 0.0)
  (Rendering|SetVisibility _effect true true)
  (Rendering|Material|SetMaterial _effect 0 "/Game/Material/Charge.Charge"))

(event EventActivateWeapon
  (Rendering|SetVisibility (Variables|Default|GetPulseGunMesh) true true))

(fn ConstructionScript)