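; Player flamethrower weapon that burns flying turret enemies and can be shown or hidden on weapon switch.
; Shoot fires once, then repeats Fire on a looping rate-based timer until release, swapping between the Flame and FlameShoot effects.
; Each Fire runs a multi-sphere trace forward from the player camera, keeps one hit per actor, then sends turrets shot and dancing-in-flames messages.
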(event Custom|Fire
  (bind _returnvalue (Game|GetPlayerCharacter 0))
  (bind _returnvalue_2 (Actor|GetComponentbyClass _returnvalue "/Script/Engine.CameraComponent"))
  (bind _returnvalue_3 (Transformation|GetWorldLocation _returnvalue_2))
  (Utilities|Array|Clear (Variables|Default|GetEnemesToCollide))
  (Utilities|Array|Clear (Variables|Default|GetEnemiesHits))
  (Components|Activation|Deactivate (Variables|Default|Getflame))
  (Components|Activation|Activate (Variables|Default|GetflameShoot) false)
  (bind _outhits (Collision|MultiSphereTraceByChannel _returnvalue_3 (+ (* (Math|Vector|GetForwardVector _returnvalue_2) (Variables|Default|GetMaxRange)) _returnvalue_3) (Variables|Default|GetFlameRadius) "TraceTypeQuery2" false (Utilities|Array|MakeArray (Game|GetPlayerCharacter 0)) "None"))
  (for _array_element _outhits
    (if (== (Utilities|Array|FindItem (Variables|Default|GetEnemesToCollide) (.HitActor (Collision|BreakHitResult _array_element))) -1)
      (Utilities|Array|Add (Variables|Default|GetEnemesToCollide) (.HitActor (Collision|BreakHitResult _array_element)))
      (Utilities|Array|Add (Variables|Default|GetEnemiesHits) _array_element)))
  (for (_array_element_2 _array_index) (Variables|Default|GetEnemesToCollide)
    (bind _asenemy_flying_turrey (Utilities|Casting|CastToEnemyFlyingTurrey _array_element_2))
    (Utilities|FlowControl|Sequence
      (:then_0
        (Class|IShootable|ReceiveShot(Message) _asenemy_flying_turrey (Utilities|Array|Get(acopy) (Variables|Default|GetEnemiesHits) _array_index)))
      (:then_1
        (Class|IShootable|DancinginFlames(Message) _asenemy_flying_turrey)))))

(event EventBeginPlay)

(event Collision|EventActorBeginOverlap
  (params (OtherActor :type Actor%20Object%20Reference)))

(event EventShoot
  (params (isZooming :type Boolean))
  ;[1 1 1] Interface shoot implementation
  (Variables|Default|SetisAiming isZooming)
  (Utilities|FlowControl|DoOnce false
    (:Completed
      (CallFunction|Fire)
      (Utilities|Time|SetTimerbyFunctionName 0 "Fire" (/ 1.0 (Variables|Default|GetRoundsPerSec)) true))))

(event EventDeactivateWeapon
  ;[1 1 1] Change weapon
  (CallFunction|ReleaseShoot)
  (Rendering|SetVisibility (Variables|Default|GetFlamethrowerMesh) false true))

(event EventReleaseShoot
  ;[1 1 1] Interface shoot implementation
  (Components|Activation|Activate (Variables|Default|Getflame) false)
  (Components|Activation|Deactivate (Variables|Default|GetflameShoot))
  (Utilities|Time|ClearTimerbyFunctionName 0 "Fire")
  (Utilities|FlowControl|DoOnce false) ; enters at Reset
)

(event EventTick
  (params (DeltaSeconds :type Float%20%28single-precision%29)))

(event EventActivateWeapon
  ;[1 1 1] Change weapon
  (CallFunction|ReleaseShoot)
  (Rendering|SetVisibility (Variables|Default|GetFlamethrowerMesh) true true))

(fn ConstructionScript)