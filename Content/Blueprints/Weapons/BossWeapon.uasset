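; Boss weapon Blueprint that fires bursts of BossProjectile actors at a target actor.
; EnemyShoot resets the bullet counter from NumBullets and calls EnemyFire, which loops through a short Delay until the burst is spent.
; Each shot spawns at ProjectileSpawnPoint, re-aims at the target's current location and plays the shoot sound there.
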(event Custom|EnemyFire
  (params (TargetToShoot :type Actor%20Object%20Reference) (Enemy :type Actor%20Object%20Reference))
  (bind _projectilespawnpoint (Variables|Default|GetProjectileSpawnPoint))
  (bind _returnvalue (Transformation|GetWorldLocation _projectilespawnpoint))
  (Game|SpawnActorfromClass "/Game/Blueprints/Weapons/BossProjectile.BossProjectile_C" (Math|Transform|MakeTransform _returnvalue (Math|Rotator|MakeRotfromX (- (Transformation|GetActorLocation TargetToShoot) _returnvalue))) "Undefined" 0 0 :!label _label)
  (Audio|SpawnSoundatLocation "/Game/Audio/shootSFX.shootSFX" (Transformation|GetWorldLocation (Variables|Default|GetProjectileSpawnPoint)))
  (Variables|Default|Setbullets (- (Variables|Default|Getbullets) 1))
  (if (> (Variables|Default|Getbullets) 0)
    (Utilities|FlowControl|Delay 0.2)
    (goto _label)))

(event EventEnemyShoot
  (params (TargetToShoot :type Actor%20Object%20Reference) (EnemyActor :type Actor%20Object%20Reference))
  (Variables|Default|Setbullets (Variables|Default|GetnumBullets))
  (CallFunction|EnemyFire TargetToShoot EnemyActor))

(fn ConstructionScript)