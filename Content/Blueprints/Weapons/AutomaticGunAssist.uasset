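; Automatic hitscan gun that fires on a looping timer with camera shake, muzzle flash and sound.
; Each shot runs a camera sphere trace sized by aim state, then a line trace with random spread when not aiming.
; Direct IShootable hits receive damage and a message, while trails, decals and particles show shots.
; The assist fallback rechecks the direct-hit actor instead of the assisted one, so it is effectively unreachable.
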(event Custom|ShootFX
  ;[1 1 1] ShootFX - MuzzleFlash + Sound
  (Audio|SpawnSoundatLocation "/Game/Audio/shootSFX.shootSFX" (Transformation|GetWorldLocation (Variables|Default|GetProjectileSpawnPoint)))
  (Components|Activation|Activate (Variables|Default|GetParticleSystem) false)
  (Utilities|FlowControl|Delay 0.1)
  (Components|Activation|Deactivate (Variables|Default|GetParticleSystem)))

(event Custom|Fire
  ;[1 1 1] Fire
  (if (Variables|Default|GetisAiming)
    (Variables|AimOffset|SetShake%20Class "/Game/Blueprints/Weapons/CameraShakes/AutomaticGun_Shake_AIM.AutomaticGun_Shake_AIM_C")
    (else
      (Variables|AimOffset|SetShake%20Class "/Game/Blueprints/Weapons/CameraShakes/AutomaticGun_Shake.AutomaticGun_Shake_C")))
  (Camera|PlayWorldCameraShake (Variables|AimOffset|GetShake%20Class) (Transformation|GetActorLocation (Game|GetPlayerCharacter 0)) 0.0 5e+02)
  (CallFunction|ShootFX)
  (Utilities|FlowControl|Delay (Variables|Default|GetshootDelay))
  (CallFunction|AimAssist))

(event Custom|AimAssist
  (bind _returnvalue (Game|GetPlayerCharacter 0))
  (bind _maxrange (Variables|Default|GetMaxRange))
  (bind _returnvalue_2 (Actor|GetComponentbyClass _returnvalue "/Script/Engine.CameraComponent"))
  (bind _returnvalue_3 (Transformation|GetWorldLocation _returnvalue_2))
  (bind _returnvalue_4 (Math|Vector|GetForwardVector _returnvalue_2))
  (bind _returnvalue_5 (* _returnvalue_4 _maxrange))
  (bind _returnvalue_6 (+ _returnvalue_3 _returnvalue_5))
  ;[1 1 1] Aim Assist
  (bind (_outhit _returnvalue_7) (Collision|SphereTraceByChannel _returnvalue_3 _returnvalue_6 (Math|Float|SelectFloat (Variables|AimAssist|GetaimAssistRadiusAiming) (Variables|AimAssist|GetaimAssistRadiusNotAiming) (Variables|Default|GetisAiming)) "TraceTypeQuery2" false (Utilities|Array|MakeArray (Game|GetPlayerCharacter 0)) "None"))
  (if _returnvalue_7
    (CallFunction|RaycastShoot _outhit)
    (else
      (CallFunction|DrawDebugRay (Transformation|GetWorldLocation (Variables|Default|GetProjectileSpawnPoint)) _returnvalue_6) ; Nothing was hit
    )))

(event Custom|RaycastShoot
  (params (aimAssistHit :type Hit%20Result%20Structure))
  (bind _returnvalue (Game|GetPlayerCharacter 0))
  (bind (_bblockinghit _binitialoverlap _time _distance _location _impactpoint _normal _impactnormal _physmat _hitactor) (Collision|BreakHitResult aimAssistHit))
  (bind _returnvalue_2 (Game|GetPlayerCharacter 0))
  (bind _maxrange (Variables|Default|GetMaxRange))
  (bind _projectilespawnpoint (Variables|Default|GetProjectileSpawnPoint))
  (bind _max_offset (Variables|AimOffset|GetMax%20Offset))
  (bind _min_offset (Variables|AimOffset|GetMin%20Offset))
  (bind _returnvalue_3 (Actor|GetComponentbyClass _returnvalue "/Script/Engine.CameraComponent"))
  (bind _returnvalue_4 (Actor|GetComponentbyClass _returnvalue_2 "/Script/Engine.CameraComponent"))
  (bind _returnvalue_5 (Transformation|GetWorldLocation _projectilespawnpoint))
  (bind _returnvalue_6 (Transformation|GetWorldLocation _returnvalue_3))
  (bind _returnvalue_7 (Math|Vector|GetForwardVector _returnvalue_4))
  (bind _returnvalue_8 (Transformation|GetWorldLocation _returnvalue_4))
  (bind _returnvalue_9 (* _returnvalue_7 _maxrange))
  (bind _returnvalue_10 (+ _returnvalue_9 _returnvalue_8))
  ;[1 1 1] RaycastShot
  (Variables|AimAssist|SetassistImpactPoint _impactpoint)
  (Variables|AimAssist|SetassistActorHit _hitactor)
  (if (Variables|Default|GetisAiming)
    (Variables|AimOffset|SetOffset%20Index 0.0)
    (else
      (Variables|AimOffset|SetOffset%20Index 1.0)))
  (bind (_outhit _returnvalue_11) (Collision|LineTraceByChannel _returnvalue_6 (+ _returnvalue_6 (* (Math|Vector|GetForwardVector _returnvalue_3) (Variables|Default|GetMaxRange)) (Math|Vector|MakeVector (* (Math|Random|RandomFloatinRange _min_offset _max_offset) (Variables|AimOffset|GetOffset%20Index)) (* (Math|Random|RandomFloatinRange _min_offset _max_offset) (Variables|AimOffset|GetOffset%20Index)) (* (Math|Random|RandomFloatinRange _min_offset _max_offset) (Variables|AimOffset|GetOffset%20Index)))) "TraceTypeQuery2" false (Utilities|Array|MakeArray (Game|GetPlayerCharacter 0)) "None"))
  (bind _output_get (Variables|AimAssist|SetdirectImpactPoint (.ImpactPoint (Collision|BreakHitResult _outhit))))
  (Development|PrintString (Utilities|String|ToString(Vector) _output_get))
  (if (and _returnvalue_11 (Utilities|DoesObjectImplementInterface (.HitActor (Collision|BreakHitResult _outhit)) "/Game/Blueprints/Characters/iShootable.iShootable_C"))
    (Class|IShootable|ReceiveShot(Message) (.HitActor (Collision|BreakHitResult _outhit)) _outhit)
    (Game|Damage|ApplyDamage (.HitActor (Collision|BreakHitResult _outhit)) (Variables|Default|Getdamage) 0 0)
    (CallFunction|DrawDebugRay (Transformation|GetWorldLocation (Variables|Default|GetProjectileSpawnPoint)) (Variables|AimAssist|GetdirectImpactPoint))
    (CallFunction|DrawFX (Variables|AimAssist|GetdirectImpactPoint) (Math|Conversions|RotationFromXVector (.ImpactNormal (Collision|BreakHitResult _outhit))))
    (elif (Utilities|DoesObjectImplementInterface (.HitActor (Collision|BreakHitResult _outhit)) "/Game/Blueprints/Characters/iShootable.iShootable_C")
      (bind (_outhit_2 _returnvalue_12) (Collision|LineTraceByChannel (Transformation|GetWorldLocation (Actor|GetComponentbyClass (Game|GetPlayerCharacter 0) "/Script/Engine.CameraComponent")) (Variables|AimAssist|GetassistImpactPoint) "TraceTypeQuery2" false (Utilities|Array|MakeArray (Game|GetPlayerCharacter 0)) "Persistent"))
      (if _returnvalue_12
        (Class|IShootable|ReceiveShot(Message) (Variables|AimAssist|GetassistActorHit) _outhit_2)
        (CallFunction|DrawDebugRay _returnvalue_5 (Variables|AimAssist|GetassistImpactPoint))
        (CallFunction|DrawFX (Variables|AimAssist|GetassistImpactPoint) (Math|Conversions|RotationFromXVector (.ImpactNormal (Collision|BreakHitResult _outhit_2))))
        (else
          (CallFunction|DrawDebugRay _returnvalue_5 _returnvalue_10)
          (CallFunction|DrawFX _returnvalue_10 "0, 0, 0")))
      (else
        (CallFunction|DrawDebugRay (Transformation|GetWorldLocation (Variables|Default|GetProjectileSpawnPoint)) (Variables|AimAssist|GetdirectImpactPoint))
        (CallFunction|DrawFX (Variables|AimAssist|GetdirectImpactPoint) "0, 0, 0")))))

(event EventReleaseShoot
  ;[1 1 1] Shoot/Release shoot event
  (Utilities|Time|ClearTimerbyFunctionName 0 "Fire")
  (Utilities|FlowControl|DoOnce false) ; enters at Reset
)

(event EventShoot
  (params (isZooming :type Boolean))
  ;[1 1 1] Shoot/Release shoot event
  (Variables|Default|SetisAiming isZooming)
  (Utilities|FlowControl|DoOnce false
    (:Completed
      (CallFunction|Fire)
      (Utilities|Time|SetTimerbyFunctionName 0 "Fire" (/ 1.0 (Variables|Default|GetRounds%20per%20sec)) true))))

(event EventDeactivateWeapon
  ;[1 1 1] Change weapon
  (CallFunction|ReleaseShoot)
  (Rendering|SetVisibility (Variables|Default|GetAutomaticGunMesh) false true))

(event EventActivateWeapon
  ;[1 1 1] Change weapon
  (CallFunction|ReleaseShoot)
  (Rendering|SetVisibility (Variables|Default|GetAutomaticGunMesh) true true))

(fn ConstructionScript)

(fn DrawDebugRay
  (params (startPos :type Vector) (endPos :type Vector))
  (Game|SpawnActorfromClass "/Game/Blueprints/Weapons/BulletTrail.BulletTrail_C" (Math|Transform|MakeTransform startPos (Math|Rotator|FindLookatRotation startPos endPos) "1,1,1") "AdjustIfPossibleButDontSpawnIfColliding" 0 0)
  ;[1 1 1] Draw debug ray
  (if (Variables|Default|GetdrawDebugRays)
    (Collision|LineTraceByChannel startPos endPos "TraceTypeQuery2" false (Utilities|Array|MakeArray (Game|GetPlayerCharacter 0)) "ForDuration")))

(fn DrawFX
  (params (location :type Vector) (rotation :type Rotator))
  (Rendering|Decal|SpawnDecalatLocation "/Game/Material/M_Decal_BulletMark.M_Decal_BulletMark" "25.000000,25.000000,25.000000" location rotation 5.0)
  (Effects|SpawnEmitteratLocation "/Game/Effects/P_BulletImpact.P_BulletImpact" location rotation))