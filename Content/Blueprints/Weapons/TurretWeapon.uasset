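; Turret weapon Blueprint that aims a sphere and cannon and fires projectiles while the trigger is held.
; Shoot fires once through a DoOnce, then loops Fire on a timer at RoundsPerSec until ReleaseShoot.
; Fire spawns a sound and a speed-set projectile at ProjectileSpawn, instigated by player pawn 0.
; AdjustRotation rate-limits sphere yaw, but the cannon snaps to its input rotation, leaving its stepped pitch unwired.
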(event Custom|Fire
  (bind _projectilespawn (Variables|Default|GetProjectileSpawn))
  (bind _projectilespeed (Variables|Default|GetProjectileSpeed))
  (bind _returnvalue (Game|SpawnActorfromClass "/Game/Blueprints/Weapons/TurretProjectile.TurretProjectile_C" (Math|Transform|MakeTransform (Transformation|GetWorldLocation _projectilespawn) (Math|Conversions|RotationFromXVector (Math|Vector|GetForwardVector _projectilespawn))) "Undefined" 0 (Game|Player|GetPlayerPawn 0)))
  (Audio|SpawnSoundatLocation 0 (Transformation|GetWorldLocation (Variables|Default|GetProjectileSpawn)))
  (Variables|/Script/Engine.ProjectileMovementComponent|SetInitialSpeed (Variables|/Game/Blueprints/Weapons/TurretProjectile.TurretProjectile_C|GetProjectileMovement _returnvalue) _projectilespeed)
  (Variables|/Script/Engine.ProjectileMovementComponent|SetMaxSpeed (Variables|/Game/Blueprints/Weapons/TurretProjectile.TurretProjectile_C|GetProjectileMovement _returnvalue) _projectilespeed))

(event Custom|RotateCannon
  (params (NewRotation :type Rotator))
  (bind _deltaangle (CallFunction|AdjustRotation (.Pitch (Math|Rotator|BreakRotator (Variables|/Script/Engine.SceneComponent|GetRelativeRotation (Variables|Default|GetCannon)))) (.Pitch (Math|Rotator|BreakRotator NewRotation)) (Variables|Default|GetCannonRotationSpeed) (Utilities|Time|GetWorldDeltaSeconds)))
  (Transformation|SetRelativeRotation (Variables|Default|GetCannon) NewRotation false false))

(event Custom|RotateSphere
  (params (NewRotation :type Rotator))
  (bind (_roll _pitch _yaw) (Math|Rotator|BreakRotator NewRotation))
  (bind _deltaangle (CallFunction|AdjustRotation (.Yaw (Math|Rotator|BreakRotator (Transformation|GetWorldRotation (Variables|Default|GetSphere)))) _yaw (Variables|Default|GetSphereRotationSpeed) (Utilities|Time|GetWorldDeltaSeconds)))
  (Transformation|SetWorldRotation (Variables|Default|GetSphere) (Math|Rotator|MakeRotator _roll _pitch _deltaangle) false false))

(event EventReleaseShoot
  (Utilities|Time|ClearTimerbyFunctionName 0 "Fire")
  (Utilities|FlowControl|DoOnce false) ; enters at Reset
)

(event EventShoot
  (Utilities|FlowControl|DoOnce false
    (:Completed
      (CallFunction|Fire)
      (Utilities|Time|SetTimerbyFunctionName 0 "Fire" (/ 1.0 (Variables|Default|GetRoundsPerSec)) true))))

(fn ConstructionScript)

(fn AdjustRotation
  (params (currentAngle :type Float%20%28single-precision%29) (targetAngle :type Float%20%28single-precision%29) (rotationSpeed :type Float%20%28single-precision%29) (deltaSeconds :type Float%20%28single-precision%29))
  (bind _returnvalue (- targetAngle currentAngle))
  (bind _returnvalue_2 (* rotationSpeed deltaSeconds))
  (return (Math|Float|SelectFloat targetAngle (Math|Float|SelectFloat (+ currentAngle _returnvalue_2) (- currentAngle _returnvalue_2) (> _returnvalue 0.0)) (< (Math|Float|Absolute(Float) _returnvalue) _returnvalue_2))))