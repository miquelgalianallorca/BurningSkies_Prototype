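; Tesla weapon Blueprint for the player: a charge-and-release hitscan gun whose ray reach grows with hold time.
; Tick builds charge and times out the ray mesh; release fires unless the player is dashing, spending ammo and starting a fire-rate cooldown.
; A camera sphere trace finds the aim point, then a muzzle trace finds the victim, destroying flying turrets and sending DisintegrateMessage.
; Reload wraps the parent's logic in a delay.
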(event Custom|DoFire
  (bind _returnvalue (Game|GetPlayerCharacter 0))
  (bind _charge (Variables|Default|GetCharge))
  (bind _timetocharge (Variables|Default|GetTimeToCharge))
  (bind _rayproyection (Variables|Default|GetRayProyection))
  (bind _range (Variables|Default|GetRange))
  (bind _projectilespawnpoint (Variables|Default|GetProjectileSpawnPoint))
  (bind _returnvalue_2 (Transformation|GetWorldLocation _projectilespawnpoint))
  (bind _returnvalue_3 (Actor|GetComponentbyClass _returnvalue "/Script/Engine.SpringArmComponent"))
  (bind _returnvalue_4 (Actor|GetComponentbyClass _returnvalue "/Script/Engine.CameraComponent"))
  (bind _returnvalue_5 (/ _charge _timetocharge))
  (bind _array (Utilities|Array|MakeArray _returnvalue))
  (bind _returnvalue_6 (Math|Vector|GetForwardVector _returnvalue_4))
  (bind _returnvalue_7 (Transformation|GetWorldLocation _returnvalue_4))
  (bind _returnvalue_8 (* _returnvalue_5 _range))
  (bind _targetarmlength (Variables|/Script/Engine.SpringArmComponent|GetTargetArmLength _returnvalue_3))
  (bind _returnvalue_9 (* _returnvalue_6 _targetarmlength))
  (bind _returnvalue_10 (* _returnvalue_6 _returnvalue_8))
  (bind _returnvalue_11 (+ _returnvalue_7 _returnvalue_9))
  (bind _returnvalue_12 (+ _returnvalue_11 _returnvalue_10))
  ;[1 1 1] Do fire
  ;;[1 0.7353 0.3083] No release during dash
  (bind _asplayer_character (Utilities|Casting|CastToPlayerCharacter (Game|GetPlayerCharacter 0)))
  (if (not (Variables|/Game/Blueprints/Characters/PlayerCharacter.PlayerCharacter_C|GetisDashing _asplayer_character))
    (bind (_outhit _returnvalue_13) (Collision|SphereTraceByChannel _returnvalue_11 _returnvalue_12 4e+01 "TraceTypeQuery2" false _array "None" true "(R=1.000000,G=0.000000,B=0.000000,A=1.000000)" "(R=0.500000,G=0.000000,B=0.000000,A=1.000000)"))
    ;;[1 1 0] Ray effect visualization
    (Transformation|SetWorldScale3D _rayproyection (Math|Vector|MakeVector 0.1875 0.1875 (* _returnvalue_8 0.0125)))
    (Transformation|SetWorldRotation _rayproyection (Math|Rotator|FindLookatRotation (Transformation|GetWorldLocation _rayproyection) (Math|Vector|SelectVector (.impactpoint _outhit) _returnvalue_12 _returnvalue_13)) false false)
    (Transformation|AddLocalRotation _rayproyection "-90.000000,0.000000,0.000000" false false)
    (Rendering|SetVisibility _rayproyection true true)
    (bind _result (Math|Integer|DecrementInt (Variables|Default|GetLoaderCurrentCapacity))
      (:%20%20
        (Variables|Default|SetisReadyToFire false)
        (Development|PrintString (Utilities|String|Append "Current ammo: " (Utilities|String|ToString(Integer) _result) " 
Backup ammo: " (Utilities|String|ToString(Integer) (Variables|Default|GetBackupCurrentCapacity))) true true "(R=0.250000,G=0.000000,B=1.000000,A=1.000000)" 5.0)
        (if _returnvalue_13
          (bind (_outhit_2 _returnvalue_14) (Collision|SphereTraceByChannel _returnvalue_2 (.impactpoint _outhit) 4e+01 "TraceTypeQuery2" false _array "None" true "(R=0.000000,G=0.000000,B=1.000000,A=1.000000)" "(R=0.000000,G=0.000000,B=0.500000,A=1.000000)"))
          (Audio|PlaySoundatLocation "/Game/Audio/Paun__online-audio-converter_com_.Paun__online-audio-converter_com_" _returnvalue_2)
          ;;[1 1 1] Hit enemy
          (if _returnvalue_14
            (if (Utilities|DoesObjectImplementInterface (.hitactor _outhit_2) "/Game/Blueprints/Enemy/EnemyDamageable.EnemyDamageable_C")
              (bind _asenemy_flying_turrey (Utilities|Casting|CastToEnemyFlyingTurrey (.hitactor _outhit_2))
                (:then
                  (Actor|DestroyActor (Variables|/Game/Blueprints/Enemy/EnemyFlyingTurrey.EnemyFlyingTurrey_C|GetEnemyWeapon _asenemy_flying_turrey))
                  (Actor|DestroyActor _asenemy_flying_turrey))
                (:CastFailed
                  _))))
          (else
            (Collision|SphereTraceByChannel _returnvalue_2 _returnvalue_12 4e+01 "TraceTypeQuery2" false _array "None" true "(R=0.000000,G=1.000000,B=0.000000,A=1.000000)" "(R=0.000000,G=0.500000,B=0.000000,A=1.000000)")))
        (Class|IKillable|Disintegrate(Message) (.hitactor _outhit_2))
        (Utilities|FlowControl|Delay (Variables|Default|GetRateOfFire))
        (Variables|Default|SetisReadyToFire true)))))

(event EventActivateWeapon
  (Rendering|SetVisibility (Variables|Default|GetSkeletalMesh) true true)
  (Rendering|SetVisibility (Variables|Default|GetRayProyection) false true))

(event EventTick
  (params (DeltaSeconds :type Float%20%28single-precision%29))
  ;[1 1 0] Ray effect visualization
  (if (Variables|/Script/Engine.SceneComponent|GetbVisible (Variables|Default|GetRayProyection))
    (bind _output_get (Variables|Default|SetTimeShowingRay (+ (Variables|Default|GetTimeShowingRay) DeltaSeconds)))
    (if (>= _output_get 0.25)
      (Rendering|SetVisibility (Variables|Default|GetRayProyection) false true)
      (Variables|Default|SetTimeShowingRay 0.0)))
  ;[1 1 1] Weapon charge
  (if (Variables|Default|GetIsCharging)
    (Variables|Default|SetCharge (Math|Float|Clamp(Float) (+ (Variables|Default|GetCharge) DeltaSeconds) 0.0 (Variables|Default|GetTimeToCharge)))))

(event EventDeactivateWeapon
  (Rendering|SetVisibility (Variables|Default|GetSkeletalMesh) false true)
  (Rendering|SetVisibility (Variables|Default|GetRayProyection) false true))

(event EventReleaseShoot
  (bind _effect (Variables|Default|GetEffect))
  ;[1 1 1] Release and shoot
  (if (Variables|Default|GetIsCharging)
    (Variables|Default|SetIsCharging false)
    (Rendering|Material|SetMaterial (Variables|Default|GetEffect) 0 "/Game/Material/Fire.Fire")
    (CallFunction|DoFire)
    (Utilities|FlowControl|Delay 0.5)
    (Rendering|Material|SetMaterial _effect 0 0)
    (Rendering|SetVisibility _effect false true)
    (Variables|Default|SetCharge 0.0)))

(event EventReload
  ;[1 1 1] Reload weapon
  (Variables|Default|SetisReadyToFire false)
  (|CallParentFunction)
  (Utilities|FlowControl|Delay (Variables|Default|GetReloadTime))
  (Variables|Default|SetisReadyToFire true)
  (Development|PrintString (Utilities|String|Append "WEAPON RELOADED 
Current ammo: " (Utilities|String|ToString(Integer) (Variables|Default|GetLoaderCurrentCapacity)) " 
Backup ammo: " (Utilities|String|ToString(Integer) (Variables|Default|GetBackupCurrentCapacity))) true true "(R=0.250000,G=0.000000,B=1.000000,A=1.000000)" 5.0))

(event EventShootBP
  (params (IsZooming :type Boolean))
  (bind _effect (Variables|Default|GetEffect))
  ;[1 1 1] Start charging
  (if (and (> (Variables|Default|GetLoaderCurrentCapacity) 0) (Variables|Default|GetisReadyToFire))
    (Variables|Default|SetIsCharging true)
    (Rendering|SetVisibility _effect true true)
    (Rendering|Material|SetMaterial _effect 0 "/Game/Material/Charge.Charge")))

(event EventSetActivationBP
  (params (Activate :type Boolean))
  ;[1 1 1] Weapon activation
  (Rendering|SetVisibility (Variables|Default|GetSkeletalMesh) Activate true)
  (Rendering|SetVisibility (Variables|Default|GetRayProyection) false true))

(event EventReleaseShootBP
  (bind _effect (Variables|Default|GetEffect))
  ;[1 1 1] Release and shoot
  (if (Variables|Default|GetIsCharging)
    (Variables|Default|SetIsCharging false)
    (Rendering|Material|SetMaterial (Variables|Default|GetEffect) 0 "/Game/Material/Fire.Fire")
    (CallFunction|DoFire)
    (Utilities|FlowControl|Delay 0.5)
    (Rendering|Material|SetMaterial _effect 0 0)
    (Rendering|SetVisibility _effect false true)
    (Variables|Default|SetCharge 0.0)))

(event EventBeginPlay
  ;[1 1 1] Init weapon
  (|CallParentFunction)
  (Variables|Default|SetLoaderCurrentCapacity (Variables|Default|GetLoaderMaxCapacity))
  (Variables|Default|SetBackupCurrentCapacity (Variables|Default|GetBackupMaxCapacity)))

(event EventShoot
  (params (isZooming :type Boolean))
  (bind _effect (Variables|Default|GetEffect))
  ;[1 1 1] Start charging
  (if (and (> (Variables|Default|GetLoaderCurrentCapacity) 0) (Variables|Default|GetisReadyToFire))
    (Variables|Default|SetIsCharging true)
    (Rendering|SetVisibility _effect true true)
    (Rendering|Material|SetMaterial _effect 0 "/Game/Material/Charge.Charge")))

(fn ConstructionScript
  (|CallParentFunction))