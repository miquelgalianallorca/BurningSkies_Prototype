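; AirTower is a destructible tower with a spinning antenna that is linked to a shield actor.
; Tick rotates the antenna pivot, and each Shot event subtracts fixed damage from health until the tower is killed.
; Kill plays explosion effects and sound, swaps the column material, removes the antenna and destroys the associated shield, then turns off the fire after a delay.
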(event EventBeginPlay
  (Variables|Life|SetCurrentHealth (Variables|Life|GetMaxHealth))
  (Variables|Life|SetIsDead false))

(event EventKill
  (Components|Activation|Activate (Variables|Default|GetExplosion) false)
  (Components|Activation|Activate (Variables|Default|GetExplosionFire) false)
  (Audio|PlaySoundatLocation "/Game/Audio/Explosion.Explosion" (Transformation|GetWorldLocation (Variables|Default|GetColumn)))
  (Rendering|Material|SetMaterial (Variables|Default|GetColumn) 0 "/Game/DemoRoom/Materials/M_DemoWall_Inst_NamePlate.M_DemoWall_Inst_NamePlate")
  (Components|DestroyComponent (Variables|Default|GetAntenna))
  (Variables|Life|SetIsDead true)
  (Actor|DestroyActor (Variables|Default|GetAssociatedShield))
  (Utilities|FlowControl|Delay 1e+01)
  (Components|Activation|Deactivate (Variables|Default|GetExplosionFire)))

(event EventTick
  (params (DeltaSeconds :type Float%20%28single-precision%29))
  (Transformation|AddLocalRotation (Variables|Default|GetAntennaPivot) (Math|Rotator|MakeRotator 0.0 0.0 (* DeltaSeconds 6e+01)) false false))

(event EventShot
  (params (Hit :type Hit%20Result%20Structure))
  (if (not (Variables|Life|GetIsDead))
    (bind _output_get (Variables|Life|SetCurrentHealth (- (Variables|Life|GetCurrentHealth) (Variables|Default|GetNormalDamage))))
    (if (<= _output_get 0.0)
      (CallFunction|Kill))))

(fn ConstructionScript)