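; Fuel station actor that recharges the player character's fuel while they stand inside its sphere trigger.
; Entering spawns an electricity arc on the station mesh, guarded by a DoOnce that resets on exit when the arc is destroyed.
; A looping 0.1-second delay retargets the beam to the player's spine and feeds a one-second delay that adds RechargeRate, capped at MaxFuel.
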(event OnComponentBeginOverlap(Sphere)
  (params (OverlappedComponent :type Primitive%20Component%20Object%20Reference) (OtherActor :type Actor%20Object%20Reference) (OtherComp :type Primitive%20Component%20Object%20Reference) (OtherBodyIndex :type Integer) (bFromSweep :type Boolean) (SweepResult :type Hit%20Result%20Structure%20%28by%20ref%29))
  (bind _returnvalue (Game|GetPlayerCharacter 0))
  (Utilities|FlowControl|DoOnce false
    (:Completed
      (bind _asplayer_character (Utilities|Casting|CastToPlayerCharacter OtherActor))
      (bind _returnvalue_2 (Effects|SpawnEmitterAttached "/Game/ExampleContent/Effects/ParticleSystems/P_electricity_arc.P_electricity_arc" (Variables|Default|GetStaticMesh) "None" "0, 0, 0" "0, 0, 0" "1.000000,1.000000,1.000000" "SnapToTarget" false))
      (Class|ParticleSystemComponent|SetBeamTargetPoint _returnvalue_2 0 (Transformation|GetSocketLocation (Variables|/Script/Engine.Character|GetMesh _returnvalue) "spine_02") :!label _label)
      (Utilities|FlowControl|Sequence
        (:then_0
          (Utilities|FlowControl|Delay 1.0)
          (if (< (+ (Variables|/Game/Blueprints/Characters/PlayerCharacter.PlayerCharacter_C|Getfuel _asplayer_character) (Variables|Default|GetRecharge%20rate)) (Variables|/Game/Blueprints/Characters/PlayerCharacter.PlayerCharacter_C|GetmaxFuel _asplayer_character))
            (Variables|/Game/Blueprints/Characters/PlayerCharacter.PlayerCharacter_C|Setfuel _asplayer_character (+ (Variables|/Game/Blueprints/Characters/PlayerCharacter.PlayerCharacter_C|Getfuel _asplayer_character) (Variables|Default|GetRecharge%20rate)))
            (else
              (Variables|/Game/Blueprints/Characters/PlayerCharacter.PlayerCharacter_C|Setfuel _asplayer_character (Variables|/Game/Blueprints/Characters/PlayerCharacter.PlayerCharacter_C|GetmaxFuel _asplayer_character)))))
        (:then_1
          (Utilities|FlowControl|Delay 0.1)
          (if (Collision|IsOverlappingActor (Variables|Default|GetSphere) _returnvalue :!class /Script/Engine.PrimitiveComponent)
            (Utilities|IsValid _returnvalue_2
              (:Is%20Valid
                (goto _label)))))))))

(event OnComponentEndOverlap(Sphere)
  (params (OverlappedComponent :type Primitive%20Component%20Object%20Reference) (OtherActor :type Actor%20Object%20Reference) (OtherComp :type Primitive%20Component%20Object%20Reference) (OtherBodyIndex :type Integer))
  (bind _returnvalue (Game|GetPlayerCharacter 0))
  (Utilities|IsValid (stale OnComponentBeginOverlap(Sphere) _returnvalue_2)
    (:Is%20Valid
      (Components|DestroyComponent (stale OnComponentBeginOverlap(Sphere) _returnvalue_2))
      (Utilities|FlowControl|DoOnce false) ; enters at Reset
    )))

(event EventBeginPlay)

(event Collision|EventActorBeginOverlap
  (params (OtherActor :type Actor%20Object%20Reference)))

(event EventTick
  (params (DeltaSeconds :type Float%20%28single-precision%29)))

(fn ConstructionScript)