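; Game mode that scripts an airship mission from jetpack pickup through shield takedown, combat, boss, artifact and exit, with optional explosives and evacuation countdown.
; BeginPlay creates compass, dialogue and objective-list HUDs, hides mission props and binds world actors' delegates.
; Those events drive progression, revealing actors, retargeting the compass, swapping PTM headlines and playing one of four dialogue sets.
; Killing all tagged enemies spawns the boss; reaching the exit pauses the game.
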(event Custom|EndMission
  ;[1 1 1] End mission
  (Game|SetGamePaused true))

(event Custom|ArtifactPicked
  ;[1 1 1] Kill boss, spawn artifact and pick artifact
  (Default|RemoveHeadline (Variables|Default|GetMissionListHUDReference) "PTM007")
  (if (Variables|Default|GetPlayerGotExplosives)
    (CallFunction|ActivateExplosivesDroppingZone))
  (CallFunction|ActivateEndMissionPoint)
  (Default|AddNewHeadline (Variables|Default|GetMissionListHUDReference) "PTM009"))

(event Custom|ItsTheFinalCountdown
  ;[1 1 1] Evacuate airship
  (Utilities|FlowControl|DoOnce false
    (:Completed
      (bind _returnvalue (UserInterface|CreateWidget "/Game/Blueprints/UI/EvacuationTimerHUD.EvacuationTimerHUD_C"))
      (bind _output_get (Variables|Default|SetEvacuationTimerHUDReference _returnvalue))
      (UserInterface|Viewport|AddtoPlayerScreen _output_get)
      (Variables|Default|SetBeginTime (Math|DateTime|Now))
      (if (not (<= (- (Variables|Default|GetEvacuationTime) (Math|Timespan|GetTotalSeconds (- (Math|DateTime|Now) (Variables|Default|GetBeginTime)))) 0.0)) :!label _label
        (Utilities|FlowControl|Delay (Utilities|Time|GetWorldDeltaSeconds))
        (Default|RefreshTimer (Variables|Default|GetEvacuationTimerHUDReference) (- (Variables|Default|GetEvacuationTime) (Math|Timespan|GetTotalSeconds (- (Math|DateTime|Now) (Variables|Default|GetBeginTime)))))
        (goto _label)))))

(event Custom|ActivateExplosivesDroppingZone
  ;[1 1 1] Activate explosives dropping zone
  (bind _outactors (Actor|GetAllActorsOfClass "/Game/Blueprints/Mission/ExplosivesDroppingZone.ExplosivesDroppingZone_C"))
  (for _array_element _outactors
    (Rendering|SetActorHiddenInGame _array_element false)
    (EventDispatchers|BindEventtoOnExplosivesDropped _array_element (delegate Custom|ActivateEvacuationTime)))
  (Default|AddNewHeadline (Variables|Default|GetMissionListHUDReference) "PTM008"))

(event Custom|ActivateEndMissionPoint
  ;[1 1 1] End mission
  (bind _outactors (Actor|GetAllActorsOfClass "/Game/Blueprints/Mission/EndMissionPoint.EndMissionPoint_C"))
  (for _array_element _outactors
    (Rendering|SetActorHiddenInGame _array_element false)
    (Default|SetNewTarget (Variables|Default|GetMissionCompassHUDReference) _array_element)
    (EventDispatchers|BindEventtoOnMissionAccomplished _array_element (delegate Custom|EndMission))))

(event Custom|ActivateEvacuationTime
  ;[1 1 1] Activate explosives dropping zone
  (Default|RemoveHeadline (Variables|Default|GetMissionListHUDReference) "PTM008")
  (CallFunction|ItstheFinalCountdown))

(event Custom|ExplosivesPicked
  ;[1 1 1] Shield destroyed
  (Variables|Default|SetPlayerGotExplosives true)
  (Default|RemoveHeadline (Variables|Default|GetMissionListHUDReference) "PTM005"))

(event Custom|ShowFirstDialogue
  ;[1 1 1] Init first mission
  (Utilities|FlowControl|Delay 1.5)
  (CallFunction|SetNewDialogue)
  (EventDispatchers|BindEventtoOnAnimationFinished (Variables|/Game/Blueprints/UI/Dialogues/FloatingDialogueHUD.FloatingDialogueHUD_C|GetUnPopUp (Variables|Default|GetDialogueHUDReference)) (delegate Custom|ActivateJetpacks)))

(event Custom|EnemyEliminated
  (params (KilledActor :type Actor%20Object%20Reference))
  (bind _bossspawner (Variables|Default|GetBossSpawner))
  (bind _enemiestoeliminate (Variables|Default|GetEnemiesToEliminate))
  (bind _missionlisthudreference (Variables|Default|GetMissionListHUDReference))
  ;[1 1 1] Combats on enemy airship
  (Utilities|Array|RemoveIndex _enemiestoeliminate (Utilities|Array|FindItem _enemiestoeliminate KilledActor))
  (if (== (Utilities|Array|Length _enemiestoeliminate) 0)
    (Default|SpawnBoss _bossspawner)
    (Default|SetNewTarget (Variables|Default|GetMissionCompassHUDReference) (Variables|/Game/Blueprints/Enemy/Bosses/BossSpawner.BossSpawner_C|GetSpawnedBoss _bossspawner))
    (Default|RemoveHeadline _missionlisthudreference "PTM003")
    (Default|AddNewHeadline _missionlisthudreference "PTM006")))

(event Custom|ShowSecondDialogue
  (bind _missionlisthudreference (Variables|Default|GetMissionListHUDReference))
  (bind _missioncompasshudreference (Variables|Default|GetMissionCompassHUDReference))
  ;[1 1 1] Show second dialogue
  (Default|RemoveHeadline _missionlisthudreference "PTM002")
  (Default|AddNewHeadline _missionlisthudreference "PTM003")
  (CallFunction|SetNewDialogue 1)
  (bind _outactors (Actor|GetAllActorsOfClass "/Game/Blueprints/Objects/Artifact.Artifact_C"))
  (if (Utilities|Array|IsValidIndex _outactors)
    (Default|SetNewTarget _missioncompasshudreference (Utilities|Array|Get(acopy) _outactors))
    (else
      (Default|SetVisible _missioncompasshudreference false))))

(event Custom|SpawnArtifact
  (bind _missionlisthudreference (Variables|Default|GetMissionListHUDReference))
  ;[1 1 1] Kill boss, spawn artifact and pick artifact
  (bind _outactors (Actor|GetAllActorsOfClass "/Game/Blueprints/Objects/Artifact.Artifact_C"))
  (if (Utilities|Array|IsValidIndex _outactors)
    (EventDispatchers|BindEventtoOnPicked (Utilities|Array|Get(acopy) _outactors) (delegate Custom|ArtifactPicked))
    (Rendering|SetActorHiddenInGame (Utilities|Array|Get(acopy) _outactors) false)
    (Default|SetNewTarget (Variables|Default|GetMissionCompassHUDReference) (Utilities|Array|Get(acopy) _outactors))
    (Default|RemoveHeadline _missionlisthudreference "PTM006")
    (Default|AddNewHeadline _missionlisthudreference "PTM007")))

(event Custom|ActivateJetpacks
  (bind _missionlisthudreference (Variables|Default|GetMissionListHUDReference))
  (bind _missioncompasshudreference (Variables|Default|GetMissionCompassHUDReference))
  ;[1 1 1] Init first mission
  (EventDispatchers|UnbindEventfromOnAnimationFinished (Variables|/Game/Blueprints/UI/Dialogues/FloatingDialogueHUD.FloatingDialogueHUD_C|GetUnPopUp (Variables|Default|GetDialogueHUDReference)) (delegate Custom|ActivateJetpacks))
  (Default|AddNewHeadline _missionlisthudreference "PTM001")
  (Default|AddNewHeadline _missionlisthudreference "PTM002")
  (bind _outactors (Actor|GetAllActorsOfClass "/Game/ExampleContent/Blueprints/Blueprints/BP_Button.BP_Button_C"))
  (for _array_element _outactors
    (Rendering|SetActorHiddenInGame _array_element false)
    (if (Utilities|String|Contains (Utilities|GetObjectName _array_element) "3")
      (Default|SetNewTarget _missioncompasshudreference _array_element)
      (Default|SetVisible _missioncompasshudreference true))))

(event Custom|ShowThirdDialogue
  (bind _missioncompasshudreference (Variables|Default|GetMissionCompassHUDReference))
  (bind _missionlisthudreference (Variables|Default|GetMissionListHUDReference))
  ;[1 1 1] Show third dialogue
  (CallFunction|SetNewDialogue 2)
  (bind _outactors (Actor|GetAllActorsOfClass "/Game/Blueprints/Objects/AirTower.AirTower_C"))
  (if (Utilities|Array|IsValidIndex _outactors)
    (Default|SetNewTarget _missioncompasshudreference (Utilities|Array|Get(acopy) _outactors))
    (else
      (Default|SetVisible _missioncompasshudreference false)))
  (Default|RemoveHeadline _missionlisthudreference "PTM003")
  (Default|AddNewHeadline _missionlisthudreference "PTM004"))

(event Custom|ShowFourthDialogue
  (bind _missionlisthudreference (Variables|Default|GetMissionListHUDReference))
  ;[1 1 1] Shield destroyed
  (CallFunction|SetNewDialogue 3)
  (Default|AddNewHeadline (Variables|Default|GetMissionListHUDReference) "PTM005")
  (bind _outactors (Actor|GetAllActorsOfClass "/Game/Blueprints/Objects/Dynamite.Dynamite_C"))
  (for _array_element _outactors
    (Rendering|SetActorHiddenInGame _array_element false)
    (EventDispatchers|BindEventtoOnPicked _array_element (delegate Custom|ExplosivesPicked)))
  (bind _outactors_2 (Actor|GetAllActorsOfClass "/Game/Blueprints/Objects/Artifact.Artifact_C"))
  (for _array_element_2 _outactors_2
    (Default|SetNewTarget (Variables|Default|GetMissionCompassHUDReference) _array_element_2))
  (Default|RemoveHeadline _missionlisthudreference "PTM004")
  (Default|AddNewHeadline _missionlisthudreference "PTM003")
  (Default|AddNewHeadline _missionlisthudreference "PTM005"))

(event Custom|SetNewDialogue
  (params (DialogueID :type Integer))
  (bind _dialoguehudreference (Variables|Default|GetDialogueHUDReference))
  ;[1 1 1] Set a new dialogue based on ID
  (switch int DialogueID
    (:0
      (Utilities|FlowControl|DoOnce false
        (:Completed
          (Variables|/Game/Blueprints/UI/Dialogues/FloatingDialogueHUD.FloatingDialogueHUD_C|SetDialogueSections _dialoguehudreference (Utilities|Array|MakeArray (Utilities|Array|Get(acopy) (Variables|Default|GetDialogueSections)) (Utilities|Array|Get(acopy) (Variables|Default|GetDialogueSections) 1) (Utilities|Array|Get(acopy) (Variables|Default|GetDialogueSections) 2) (Utilities|Array|Get(acopy) (Variables|Default|GetDialogueSections) 3) (Utilities|Array|Get(acopy) (Variables|Default|GetDialogueSections) 4))))))
    (:1
      (Utilities|FlowControl|DoOnce false
        (:Completed
          (Variables|/Game/Blueprints/UI/Dialogues/FloatingDialogueHUD.FloatingDialogueHUD_C|SetDialogueSections _dialoguehudreference (Utilities|Array|MakeArray (Utilities|Array|Get(acopy) (Variables|Default|GetDialogueSections) 5))))))
    (:2
      (Utilities|FlowControl|DoOnce false
        (:Completed
          (Variables|/Game/Blueprints/UI/Dialogues/FloatingDialogueHUD.FloatingDialogueHUD_C|SetDialogueSections _dialoguehudreference (Utilities|Array|MakeArray (Utilities|Array|Get(acopy) (Variables|Default|GetDialogueSections) 6) (Utilities|Array|Get(acopy) (Variables|Default|GetDialogueSections) 7) (Utilities|Array|Get(acopy) (Variables|Default|GetDialogueSections) 8) (Utilities|Array|Get(acopy) (Variables|Default|GetDialogueSections) 9))))))
    (:3
      (Utilities|FlowControl|DoOnce false
        (:Completed
          (Variables|/Game/Blueprints/UI/Dialogues/FloatingDialogueHUD.FloatingDialogueHUD_C|SetDialogueSections _dialoguehudreference (Utilities|Array|MakeArray (Utilities|Array|Get(acopy) (Variables|Default|GetDialogueSections) 10) (Utilities|Array|Get(acopy) (Variables|Default|GetDialogueSections) 11) (Utilities|Array|Get(acopy) (Variables|Default|GetDialogueSections) 12) (Utilities|Array|Get(acopy) (Variables|Default|GetDialogueSections) 13) (Utilities|Array|Get(acopy) (Variables|Default|GetDialogueSections) 14)))))))
  (Default|InitDialogue _dialoguehudreference))

(event EventBeginPlay
  (bind _returnvalue (Game|GetPlayerController 0))
  (bind _enemiestoeliminate (Variables|Default|GetEnemiesToEliminate))
  ;[1 1 1] Get BossSpawner reference
  (bind _outactors (Actor|GetAllActorsOfClass "/Game/Blueprints/Enemy/Bosses/BossSpawner.BossSpawner_C"))
  (if (Utilities|Array|IsValidIndex _outactors)
    (Variables|Default|SetBossSpawner (Utilities|Array|Get(acopy) _outactors)))
  ;[1 1 1] Spawn HUDs
  (bind _returnvalue_2 (UserInterface|CreateWidget "/Game/Blueprints/UI/MissionCompassHUD.MissionCompassHUD_C"))
  (bind _output_get (Variables|Default|SetMissionCompassHUDReference _returnvalue_2))
  (UserInterface|Viewport|AddtoPlayerScreen _output_get)
  (bind _returnvalue_3 (UserInterface|CreateWidget "/Game/Blueprints/UI/Dialogues/FloatingDialogueHUD.FloatingDialogueHUD_C" _returnvalue))
  (bind _output_get_2 (Variables|Default|SetDialogueHUDReference _returnvalue_3))
  (UserInterface|Viewport|AddtoPlayerScreen _output_get_2)
  (bind _returnvalue_4 (UserInterface|CreateWidget "/Game/Blueprints/UI/Dialogues/MissionHeadlineListHUD.MissionHeadlineListHUD_C" _returnvalue))
  (bind _output_get_3 (Variables|Default|SetMissionListHUDReference _returnvalue_4))
  (UserInterface|Viewport|AddtoPlayerScreen _output_get_3)
  ;[1 1 1] Pickup Jetpack
  (bind _outactors_2 (Actor|GetAllActorsOfClass "/Game/ExampleContent/Blueprints/Blueprints/BP_Button.BP_Button_C"))
  (if (> (Utilities|Array|Length _outactors_2) 0)
    (for _array_element _outactors_2
      (EventDispatchers|UnbindallEventsfromOnPlayerChoseJetpack _array_element)
      (EventDispatchers|BindEventtoOnPlayerChoseJetpack _array_element (delegate Custom|ShowSecondDialogue))
      ;[1 1 1] Shield detection
      (bind _outactors_3 (Actor|GetAllActorsOfClass "/Game/Blueprints/Mission/ShipShield.ShipShield_C"))
      (if (> (Utilities|Array|Length _outactors_3) 0)
        (EventDispatchers|BindEventtoOnPlayerEnteredTrigger (Utilities|Array|Get(acopy) _outactors_3) (delegate Custom|ShowThirdDialogue))
        ;[1 1 1] Shield destroyed
        (EventDispatchers|UnbindallEventsfromOnDeactivated (Utilities|Array|Get(acopy) _outactors_3))
        (EventDispatchers|BindEventtoOnDeactivated (Utilities|Array|Get(acopy) _outactors_3) (delegate Custom|ShowFourthDialogue)))
      ;[1 1 1] Combats on enemy airship
      (Utilities|Array|Clear (Variables|Default|GetEnemiesToEliminate))
      (bind _outactors_4 (Actor|GetAllActorswithTag "PTM003"))
      (for _array_element_2 _outactors_4
        (bind _asenemy_chaser (Utilities|Casting|CastToEnemy_Chaser _array_element_2)
          (:then
            (Utilities|Array|Add _enemiestoeliminate _asenemy_chaser)
            (EventDispatchers|BindEventtoOnKilled _asenemy_chaser (delegate Custom|EnemyEliminated)))
          (:CastFailed
            (bind _asquad_turret (Utilities|Casting|CastToQuadTurret _array_element_2))
            (Utilities|Array|Add _enemiestoeliminate _asquad_turret)
            (EventDispatchers|BindEventtoOnKilled _asquad_turret (delegate Custom|EnemyEliminated)))))
      ;[1 1 1] Kill boss, spawn artifact and pick artifact
      (EventDispatchers|BindEventtoOnBossKilled (Variables|Default|GetBossSpawner) (delegate Custom|SpawnArtifact))
      ;[1 1 1] Hide elements at start
      (bind _outactors_5 (Actor|GetAllActorsOfClass "/Game/ExampleContent/Blueprints/Blueprints/BP_Button.BP_Button_C"))
      (for _array_element_3 _outactors_5
        (Rendering|SetActorHiddenInGame _array_element_3 true))
      (bind _outactors_6 (Actor|GetAllActorsOfClass "/Game/Blueprints/Objects/Dynamite.Dynamite_C"))
      (for _array_element_4 _outactors_6
        (Rendering|SetActorHiddenInGame _array_element_4 true))
      (bind _outactors_7 (Actor|GetAllActorsOfClass "/Game/Blueprints/Mission/EndMissionPoint.EndMissionPoint_C"))
      (for _array_element_5 _outactors_7
        (Rendering|SetActorHiddenInGame _array_element_5 true))
      (bind _outactors_8 (Actor|GetAllActorsOfClass "/Game/Blueprints/Mission/ExplosivesDroppingZone.ExplosivesDroppingZone_C"))
      (for _array_element_6 _outactors_8
        (Rendering|SetActorHiddenInGame _array_element_6 true))
      (CallFunction|ShowFirstDialogue)))
  (bind _outactors_9 (Actor|GetAllActorsOfClass "/Game/Blueprints/Mission/ShipShield.ShipShield_C"))
  (if (> (Utilities|Array|Length _outactors_9) 0)
    (EventDispatchers|BindEventtoOnPlayerEnteredTrigger (Utilities|Array|Get(acopy) _outactors_9) (delegate Custom|ShowThirdDialogue))
    (EventDispatchers|UnbindallEventsfromOnDeactivated (Utilities|Array|Get(acopy) _outactors_9))
    (EventDispatchers|BindEventtoOnDeactivated (Utilities|Array|Get(acopy) _outactors_9) (delegate Custom|ShowFourthDialogue)))
  (Utilities|Array|Clear (Variables|Default|GetEnemiesToEliminate))
  (bind _outactors_10 (Actor|GetAllActorswithTag "PTM003"))
  (for _array_element_7 _outactors_10
    (bind _asenemy_chaser_2 (Utilities|Casting|CastToEnemy_Chaser _array_element_7)
      (:then
        (Utilities|Array|Add _enemiestoeliminate _asenemy_chaser_2)
        (EventDispatchers|BindEventtoOnKilled _asenemy_chaser_2 (delegate Custom|EnemyEliminated)))
      (:CastFailed
        (bind _asquad_turret_2 (Utilities|Casting|CastToQuadTurret _array_element_7))
        (Utilities|Array|Add _enemiestoeliminate _asquad_turret_2)
        (EventDispatchers|BindEventtoOnKilled _asquad_turret_2 (delegate Custom|EnemyEliminated)))))
  (EventDispatchers|BindEventtoOnBossKilled (Variables|Default|GetBossSpawner) (delegate Custom|SpawnArtifact))
  (bind _outactors_11 (Actor|GetAllActorsOfClass "/Game/ExampleContent/Blueprints/Blueprints/BP_Button.BP_Button_C"))
  (for _array_element_8 _outactors_11
    (Rendering|SetActorHiddenInGame _array_element_8 true))
  (bind _outactors_12 (Actor|GetAllActorsOfClass "/Game/Blueprints/Objects/Dynamite.Dynamite_C"))
  (for _array_element_9 _outactors_12
    (Rendering|SetActorHiddenInGame _array_element_9 true))
  (bind _outactors_13 (Actor|GetAllActorsOfClass "/Game/Blueprints/Mission/EndMissionPoint.EndMissionPoint_C"))
  (for _array_element_10 _outactors_13
    (Rendering|SetActorHiddenInGame _array_element_10 true))
  (bind _outactors_14 (Actor|GetAllActorsOfClass "/Game/Blueprints/Mission/ExplosivesDroppingZone.ExplosivesDroppingZone_C"))
  (for _array_element_11 _outactors_14
    (Rendering|SetActorHiddenInGame _array_element_11 true))
  (CallFunction|ShowFirstDialogue))

(fn ConstructionScript)

(fn SpawnBoss
  (bind _bossspawner (Variables|Default|GetBossSpawner))
  (Default|SpawnBoss _bossspawner)
  (Default|SetNewTarget (Variables|Default|GetMissionCompassHUDReference) _bossspawner))