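; Actor component that gives its owner a timed heal skill.
; Heal sets a healing flag and a one-shot timer that restores a number of life slots through the owner's HealthComp, then calls EndHeal.
; EndHeal clears the timer and flag, so calling it early cancels the pending heal.
; Start and end also toggle IsHealing on player 0's PlayerAnimBP, regardless of which actor owns the component.
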(event Custom|Heal
  ;[1 1 1] Heal start
  (Variables|Default|SetisHealing true)
  (bind _returnvalue (Utilities|Time|SetTimerbyEvent (delegate Custom|HealEvent) (Variables|Default|GethealingTime)))
  (Variables|Default|SettimerHandle _returnvalue)
  (CallFunction|HealAnimStart))

(event Custom|HealAnimStart
  ;[1 1 1] Animation
  (bind _asplayer_anim_bp (Utilities|Casting|CastToPlayerAnimBP (Components|SkeletalMesh|GetAnimInstance (Variables|/Script/Engine.Character|GetMesh (Game|GetPlayerCharacter 0)))))
  (Variables|/Game/Mannequin/Animations/PlayerAnimBP.PlayerAnimBP_C|SetisHealing _asplayer_anim_bp true))

(event Custom|HealEvent
  (bind _returnvalue (Components|GetOwner))
  (bind _returnvalue_2 (Actor|GetComponentbyClass _returnvalue "/Game/Blueprints/Characters/HealthComp.HealthComp_C"))
  ;[1 1 1] Heal
  (if (Utilities|IsValid _returnvalue_2)
    (Default|Heal _returnvalue_2 (* (Variables|Default|GetnHealSlots) (Variables|/Game/Blueprints/Characters/HealthComp.HealthComp_C|GetlifePerSlot _returnvalue_2)))
    (CallFunction|EndHeal)))

(event Custom|HealAnimEnd
  ;[1 1 1] Animation
  (bind _asplayer_anim_bp (Utilities|Casting|CastToPlayerAnimBP (Components|SkeletalMesh|GetAnimInstance (Variables|/Script/Engine.Character|GetMesh (Game|GetPlayerCharacter 0)))))
  (Variables|/Game/Mannequin/Animations/PlayerAnimBP.PlayerAnimBP_C|SetisHealing _asplayer_anim_bp false))

(event Custom|EndHeal
  ;[1 1 1] Heal end
  (Utilities|Time|ClearandInvalidateTimerbyHandle (Variables|Default|GettimerHandle))
  (Variables|Default|SetisHealing false)
  (CallFunction|HealAnimEnd))