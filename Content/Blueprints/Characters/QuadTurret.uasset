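; Quad-barrel turret that turns toward a nearby player and rotates through four gun positions.
; DetectPlayer sphere-overlaps pawns around the active gun, snaps the actor to face the first PlayerCharacter found and reports whether one was in range.
; Fire only advances the active gun index, wrapping after the fourth, and GetActiveGun maps that index to one of four Arrow components.
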(fn ConstructionScript)

(fn DetectPlayer
  (bind _outactors (Collision|SphereOverlapActors (Transformation|GetWorldLocation (CallFunction|GetActiveGun)) (Variables|Default|GetdetectRange) (Utilities|Array|MakeArray "ObjectTypeQuery3") "/Game/Blueprints/Characters/PlayerCharacter.PlayerCharacter_C"))
  (bind _array_element (Utilities|Array|ForEachLoopwithBreak _outactors)
    (:LoopBody
      ;[1 1 1] Face Player
      (Transformation|SetActorRotation (Math|Rotator|FindLookatRotation (Transformation|GetActorLocation) (Transformation|GetActorLocation _array_element)))
      (return true))
    (:Completed
      (return false))))

(fn Fire
  ;[1 1 1] Change active gun
  (bind _result (Math|Integer|IncrementInt (Variables|Default|GetactiveGun))
    (:%20%20
      (if (>= _result 4)
        (Variables|Default|SetactiveGun 0)))))

(fn GetActiveGun
  (return (Utilities|Select :Index (Variables|Default|GetactiveGun) :Option%200 (Variables|Default|GetArrow0) :Option%201 (Variables|Default|GetArrow1) :Option%202 (Variables|Default|GetArrow2) :Option%203 (Variables|Default|GetArrow3))))