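; MoveBobaComponent is a movement component that moves its owning PrototypeCharacter relative to that character's follow camera.
; MoveForward and MoveSide each cast the owner to PrototypeCharacter and pass an axis value to AddMovementInput along the FollowCamera's forward or right vector.
; The camera vectors are used directly, without flattening pitch or roll.
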(fn MoveForward
  (params (axisValue :type Float%20%28single-precision%29))
  (bind _asprototype_character (Utilities|Casting|CastToPrototypeCharacter (Components|GetOwner)))
  (Pawn|Input|AddMovementInput _asprototype_character (Math|Vector|GetForwardVector (Variables|/Game/Blueprints/Characters/PrototypeCharacter.PrototypeCharacter_C|GetFollowCamera _asprototype_character)) axisValue false)
  (return))

(fn MoveSide
  (params (axisValue :type Float%20%28single-precision%29))
  (bind _asprototype_character (Utilities|Casting|CastToPrototypeCharacter (Components|GetOwner)))
  (Pawn|Input|AddMovementInput _asprototype_character (Math|Vector|GetRightVector (Variables|/Game/Blueprints/Characters/PrototypeCharacter.PrototypeCharacter_C|GetFollowCamera _asprototype_character)) axisValue false)
  (return))