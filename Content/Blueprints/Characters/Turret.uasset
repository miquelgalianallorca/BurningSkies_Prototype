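; Turret actor that detects player-controlled pawns within a vision sphere and fires a spawned weapon at them.
; On begin play it spawns the TurretWeapon at a spawn point and passes it projectile, fire-rate and rotation speeds.
; Each tick it leads the target using frame-delta velocity and projectile travel time, sending yaw to the weapon's sphere and pitch to its cannon.
; It releases the trigger without a target.
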(event EventBeginPlay
  (Components|Sphere|SetSphereRadius (Variables|Default|GetVisionSphere) (Variables|Default|GetVisionRadius) true)
  (bind _returnvalue (Game|SpawnActorfromClass "/Game/Blueprints/Weapons/TurretWeapon.TurretWeapon_C" (Transformation|GetWorldTransform (Variables|Default|GetWeaponSpawn)) "Undefined" 0 0))
  (bind _output_get (Variables|Default|SetWeapon _returnvalue))
  (Variables|/Game/Blueprints/Weapons/TurretWeapon.TurretWeapon_C|SetProjectileSpeed _returnvalue (Variables|Default|GetProjectileSpeed))
  (Variables|/Game/Blueprints/Weapons/TurretWeapon.TurretWeapon_C|SetRoundsPerSec _returnvalue (Variables|Default|GetRoundsPerSecond))
  (Variables|Default|SetWeaponLocation (Transformation|GetActorLocation _output_get))
  (Variables|/Game/Blueprints/Weapons/TurretWeapon.TurretWeapon_C|SetSphereRotationSpeed _returnvalue (Variables|Default|GetSphereRotationSpeed))
  (Variables|/Game/Blueprints/Weapons/TurretWeapon.TurretWeapon_C|SetCannonRotationSpeed _returnvalue (Variables|Default|GetCannonRotationSpeed)))

(event Collision|EventActorBeginOverlap
  (params (OtherActor :type Actor%20Object%20Reference))
  (bind _aspawn (Utilities|Casting|CastToPawn OtherActor))
  (if (Pawn|IsPlayerControlled _aspawn)
    (Variables|Default|SetCurrentTarget _aspawn)))

(event EventTick
  (params (DeltaSeconds :type Float%20%28single-precision%29))
  (bind _weaponlocation (Variables|Default|GetWeaponLocation))
  (bind (_x _y _z) (Math|Vector|BreakVector _weaponlocation))
  (Utilities|IsValid (Variables|Default|GetCurrentTarget)
    (:Is%20Valid
      (Variables|Default|SetTargetLastLocation (Variables|Default|GetTargetCurrentLocation))
      (Variables|Default|SetTargetCurrentLocation (Transformation|GetActorLocation (Variables|Default|GetCurrentTarget)))
      (bind _asturret_weapon (Utilities|Casting|CastToTurretWeapon (Variables|Default|GetWeapon)))
      (Default|RotateSphere _asturret_weapon (Math|Rotator|FindLookatRotation _weaponlocation (Math|Vector|MakeVector (.x (+ (* (/ (- (Variables|Default|GetTargetCurrentLocation) (Variables|Default|GetTargetLastLocation)) DeltaSeconds) (/ (Math|Vector|VectorLength (- (Variables|Default|GetTargetCurrentLocation) (Variables|Default|GetWeaponLocation))) (Variables|Default|GetProjectileSpeed))) (Variables|Default|GetTargetCurrentLocation))) (.y (+ (* (/ (- (Variables|Default|GetTargetCurrentLocation) (Variables|Default|GetTargetLastLocation)) DeltaSeconds) (/ (Math|Vector|VectorLength (- (Variables|Default|GetTargetCurrentLocation) (Variables|Default|GetWeaponLocation))) (Variables|Default|GetProjectileSpeed))) (Variables|Default|GetTargetCurrentLocation))) _z)))
      (Default|RotateCannon _asturret_weapon (Math|Rotator|MakeRotator 0.0 (- (Class|KismetMathLibrary|DegAtan2 (- (.z (+ (* (/ (- (Variables|Default|GetTargetCurrentLocation) (Variables|Default|GetTargetLastLocation)) DeltaSeconds) (/ (Math|Vector|VectorLength (- (Variables|Default|GetTargetCurrentLocation) (Variables|Default|GetWeaponLocation))) (Variables|Default|GetProjectileSpeed))) (Variables|Default|GetTargetCurrentLocation))) _z) (Math|Vector2D|Vector2DLength (- (Math|Vector2D|MakeVector2D (.x (+ (* (/ (- (Variables|Default|GetTargetCurrentLocation) (Variables|Default|GetTargetLastLocation)) DeltaSeconds) (/ (Math|Vector|VectorLength (- (Variables|Default|GetTargetCurrentLocation) (Variables|Default|GetWeaponLocation))) (Variables|Default|GetProjectileSpeed))) (Variables|Default|GetTargetCurrentLocation))) (.y (+ (* (/ (- (Variables|Default|GetTargetCurrentLocation) (Variables|Default|GetTargetLastLocation)) DeltaSeconds) (/ (Math|Vector|VectorLength (- (Variables|Default|GetTargetCurrentLocation) (Variables|Default|GetWeaponLocation))) (Variables|Default|GetProjectileSpeed))) (Variables|Default|GetTargetCurrentLocation)))) (Math|Vector2D|MakeVector2D _x _y)))) 9e+01) 0.0))
      (Class|Weapon|Shoot(Message) (Variables|Default|GetWeapon)))
    (:Is%20Not%20Valid
      (Class|Weapon|ReleaseShoot(Message) (Variables|Default|GetWeapon)))))

(event Collision|EventActorEndOverlap
  (params (OtherActor :type Actor%20Object%20Reference))
  (bind _aspawn (Utilities|Casting|CastToPawn OtherActor))
  (if (Pawn|IsPlayerControlled _aspawn)
    (Variables|Default|SetCurrentTarget 0)))

(fn ConstructionScript)