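; Health component that tracks character life as a pool divided into equal slots, with delayed regeneration after damage.
; ReceiveDamage lowers life, resets the regeneration delay and caps auto-heal at the top of the current slot, so emptied slots stay lost.
; A looping timer started at BeginPlay counts that delay, then heals gradually until the cap.
; Heal and FillLife restore life directly, and SetLifeSlots recomputes maximum life.
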(event Custom|AutoHealTick
  ;[1 1 1] Update
  (if (Variables|AutoHeal|GetautoHealEnabled)
    ;;[1 0.7353 0.3083] Autoheal
    (bind _remaininglife (CallFunction|Heal (* (Variables|AutoHeal|GetautoHealAmountPerSec) (Variables|AutoHeal|GetautoHealDeltaTime))))
    ;;[1 0.7353 0.3083] Autoheal end
    (if (>= _remaininglife (Variables|AutoHeal|GetautoHealLimit))
      (Variables|AutoHeal|SetautoHealEnabled false))
    (else
      (bind _output_get (Variables|AutoHeal|SetautoHealTimer (+ (Variables|AutoHeal|GetautoHealTimer) (Variables|AutoHeal|GetautoHealDeltaTime))))
      (if (>= _output_get (Variables|AutoHeal|GetautoHealActivateTime))
        ;;[1 0.7353 0.3083] Autoheal start
        (if (< (Variables|Default|GetcurrentLife) (Variables|AutoHeal|GetautoHealLimit))
          (Variables|AutoHeal|SetautoHealEnabled true))))))

(event EventBeginPlay
  ;[1 1 1] Begin
  (CallFunction|SetLifeSlots (Variables|Default|GetnSlots))
  (CallFunction|FillLife)
  (Utilities|Time|SetTimerbyEvent (delegate Custom|AutoHealTick) (Variables|AutoHeal|GetautoHealDeltaTime) true))

(fn SetLifeSlots
  (params (newLifeSlots :type Integer))
  (bind _output_get (Variables|Default|SetnSlots newLifeSlots))
  (Variables|Default|SetmaxLife (* _output_get (Variables|Default|GetlifePerSlot))))

(fn ReceiveDamage
  (params (damageReceived :type Float%20%28single-precision%29))
  (bind _currentslot (CallFunction|GetCurrentSlot))
  (bind _lifeperslot (Variables|Default|GetlifePerSlot))
  (bind _returnvalue (+ _currentslot 1))
  (bind _returnvalue_2 (* _returnvalue _lifeperslot))
  (Variables|AutoHeal|SetautoHealEnabled false) ; Interrupt autoheal
  (Variables|AutoHeal|SetautoHealTimer 0.0) ; Reset autoheal timer
  (bind _output_get (Variables|Default|SetcurrentLife (Math|Float|Clamp(Float) (- (Variables|Default|GetcurrentLife) damageReceived) 0.0 (- (Variables|Default|GetcurrentLife) damageReceived))))
  (Variables|AutoHeal|SetautoHealLimit (Math|Float|Clamp(Float) _returnvalue_2 _returnvalue_2 (Variables|Default|GetmaxLife)))
  (return _output_get))

(fn FillLife
  (Variables|Default|SetcurrentLife (Variables|Default|GetmaxLife)))

(fn Heal
  (params (healAmount :type Float%20%28single-precision%29))
  (bind _output_get (Variables|Default|SetcurrentLife (Math|Float|Clamp(Float) (+ healAmount (Variables|Default|GetcurrentLife)) (+ healAmount (Variables|Default|GetcurrentLife)) (Variables|Default|GetmaxLife))))
  (return _output_get))

(fn GetCurrentSlot
  (return (Math|Float|Truncate (* (Variables|Default|GetnSlots) (/ (Variables|Default|GetcurrentLife) (Variables|Default|GetmaxLife))))))