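; Player character component that owns the four-weapon loadout and handles switching between weapons.
; LoadWeapons spawns each gun onto the mesh's Weapon socket, with only the automatic gun left visible.
; Up, down and direct-index switches wrap or jump through the array, messaging weapons to deactivate and activate.
; A timer separates tap from hold: tapping cycles forward, holding opens the weapon wheel with mouse cursor and look input ignored until release.
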(event EventBeginPlay
  (bind _asplayer_character (Utilities|Casting|CastToPlayerCharacter (Components|GetOwner)))
  (Variables|Default|SetplayerCharacter _asplayer_character))

(fn ChangeWeaponUp
  (bind _weaponindex (Variables|Default|GetweaponIndex))
  (if (== _weaponindex 3)
    (Keyboard|ChangeWeaponKey)
    (else
      (Keyboard|ChangeWeaponKey (+ _weaponindex 1)))))

(fn ChangeWeaponDown
  (bind _weaponindex (Variables|Default|GetweaponIndex))
  (if (== _weaponindex 0)
    (Keyboard|ChangeWeaponKey 3)
    (else
      (Keyboard|ChangeWeaponKey (- _weaponindex 1)))))

(fn ChangeWeaponPressed
  (bind _returnvalue (Utilities|Time|SetTimerbyFunctionName self "OpenWeaponWheel" (Variables|Default|GetholdingTimeForWeaponWheel)))
  (Variables|Default|SetweaponWheelHandle _returnvalue))

(fn OpenWeaponWheel
  (bind _returnvalue (Game|GetPlayerController 0))
  (Variables|/Game/Blueprints/Characters/PlayerCharacter.PlayerCharacter_C|SetWheelIsOpened? (Variables|Default|GetplayerCharacter) true)
  (bind _returnvalue_2 (UserInterface|CreateWidget "/Game/Blueprints/UI/WeaponsWheel/Wheel.Wheel_C"))
  (Default|SetSelectedWeaponIndex _returnvalue_2 (Variables|Default|GetweaponIndex))
  (bind _output_get (Variables|Default|SetwheelReference _returnvalue_2))
  (UserInterface|Viewport|AddtoViewport _output_get 0)
  (Variables|/Script/Engine.PlayerController|SetbShowMouseCursor _returnvalue true)
  (Input|SetIgnoreLookInput _returnvalue true)
  (Input|SetInputModeGameandUI _returnvalue _output_get "DoNotLock" true))

(fn ChangeWeaponReleased
  (bind _returnvalue (Game|GetPlayerController 0))
  (bind _playercharacter (Variables|Default|GetplayerCharacter))
  (Utilities|Time|ClearandInvalidateTimerbyHandle (Variables|Default|GetweaponWheelHandle))
  (if (not (Variables|/Game/Blueprints/Characters/PlayerCharacter.PlayerCharacter_C|GetWheelIsOpened? _playercharacter))
    (Class|Weapon|DeactivateWeapon(Message) (Variables|/Game/Blueprints/Characters/PlayerCharacter.PlayerCharacter_C|GetActualWeapon _playercharacter))
    (if (< (Variables|Default|GetweaponIndex) 3)
      (Variables|Default|SetweaponIndex (+ (Variables|Default|GetweaponIndex) 1))
      (else
        (Variables|Default|SetweaponIndex 0)))
    (bind _output_get (Variables|/Game/Blueprints/Characters/PlayerCharacter.PlayerCharacter_C|SetActualWeapon (Variables|Default|GetplayerCharacter) (Utilities|Array|Get(acopy) (Variables|Default|Getweapons) (Variables|Default|GetweaponIndex))))
    (Class|Weapon|ActivateWeapon(Message) _output_get)
    (else
      (Variables|/Game/Blueprints/Characters/PlayerCharacter.PlayerCharacter_C|SetWheelIsOpened? (Variables|Default|GetplayerCharacter) false)
      (Widget|RemovefromParent (Variables|Default|GetwheelReference))
      (Variables|/Script/Engine.PlayerController|SetbShowMouseCursor _returnvalue false)
      (Input|SetIgnoreLookInput _returnvalue false)
      (Input|SetInputModeGameOnly _returnvalue))))

(fn ChangeWeaponKey
  (params (weaponNumber :type Integer))
  (bind _playercharacter (Variables|Default|GetplayerCharacter))
  (Class|Weapon|DeactivateWeapon(Message) (Variables|/Game/Blueprints/Characters/PlayerCharacter.PlayerCharacter_C|GetActualWeapon _playercharacter))
  (Variables|Default|SetweaponIndex weaponNumber)
  (bind _output_get (Variables|/Game/Blueprints/Characters/PlayerCharacter.PlayerCharacter_C|SetActualWeapon _playercharacter (Utilities|Array|Get(acopy) (Variables|Default|Getweapons) weaponNumber)))
  (Class|Weapon|ActivateWeapon(Message) _output_get))

(fn LoadWeapons
  (bind _playercharacter (Variables|Default|GetplayerCharacter))
  ;[1 1 1] Automatic Gun
  (bind _returnvalue (Game|SpawnActorfromClass "/Game/Blueprints/Weapons/AutomaticGun.AutomaticGun_C" (Transformation|GetActorTransform (Components|GetOwner)) "Undefined" 0 0))
  (bind _output_get (Variables|/Game/Blueprints/Characters/PlayerCharacter.PlayerCharacter_C|SetActualWeapon _playercharacter _returnvalue))
  (Class|Weapon|ActivateWeapon(Message) _output_get)
  (Transformation|AttachComponentToComponent _output_get (Variables|/Script/Engine.Character|GetMesh _playercharacter) "Weapon" "SnapToTarget" "KeepRelative" "KeepRelative" true)
  (Utilities|Array|Add (Variables|Default|GetWeapons) _output_get)
  ;[1 1 1] Tesla
  (bind _returnvalue_2 (Game|SpawnActorfromClass "/Game/Blueprints/Weapons/TeslaWeapon.TeslaWeapon_C" (Transformation|GetActorTransform (Components|GetOwner)) "Undefined" 0 0))
  (Transformation|AttachComponentToComponent _returnvalue_2 (Variables|/Script/Engine.Character|GetMesh (Variables|Default|GetplayerCharacter)) "Weapon" "SnapToTarget" "KeepRelative" "KeepRelative" true)
  (Rendering|SetVisibility (Variables|/Script/Engine.Actor|GetRootComponent _returnvalue_2) false true)
  (Utilities|Array|Add (Variables|Default|GetWeapons) _returnvalue_2)
  ;[1 1 1] Flamethrower
  (bind _returnvalue_3 (Game|SpawnActorfromClass "/Game/Blueprints/Weapons/Flamethrower.Flamethrower_C" (Transformation|GetActorTransform (Components|GetOwner)) "Undefined" 0 0))
  (Transformation|AttachComponentToComponent _returnvalue_3 (Variables|/Script/Engine.Character|GetMesh (Variables|Default|GetplayerCharacter)) "Weapon" "SnapToTarget" "KeepRelative" "KeepRelative" true)
  (Rendering|SetVisibility (Variables|/Script/Engine.Actor|GetRootComponent _returnvalue_3) false true)
  (Utilities|Array|Add (Variables|Default|GetWeapons) _returnvalue_3)
  ;[1 1 1] Rocket launcher
  (bind _returnvalue_4 (Game|SpawnActorfromClass "/Game/Blueprints/Weapons/RocketLauncher.RocketLauncher_C" (Transformation|GetActorTransform (Components|GetOwner)) "Undefined" 0 0))
  (Transformation|AttachComponentToComponent _returnvalue_4 (Variables|/Script/Engine.Character|GetMesh (Variables|Default|GetplayerCharacter)) "Weapon" "SnapToTarget" "KeepRelative" "KeepRelative" true)
  (Rendering|SetVisibility (Variables|/Script/Engine.Actor|GetRootComponent _returnvalue_4) false true)
  (Utilities|Array|Add (Variables|Default|GetWeapons) _returnvalue_4))