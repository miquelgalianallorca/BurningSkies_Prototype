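; MoveGroundComponent is a component that applies planar forward and sideways movement input to its owning PrototypeCharacter.
; MoveForward and MoveSide each take an axis value and pass it as the scale to AddMovementInput, stopping if the owner cast fails.
; Direction comes from the control rotation's yaw alone, with pitch and roll zeroed so looking up or down does not tilt movement.
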(fn MoveForward
  (params (axisValue :type Float%20%28single-precision%29))
  (bind _asprototype_character (Utilities|Casting|CastToPrototypeCharacter (Components|GetOwner)))
  (Pawn|Input|AddMovementInput _asprototype_character (Math|Vector|GetForwardVector (Math|Rotator|MakeRotator 0.0 0.0 (.Yaw (Math|Rotator|BreakRotator (Pawn|GetControlRotation _asprototype_character :!class /Script/Engine.Pawn))))) axisValue false)
  (return))

(fn MoveSide
  (params (axisValue :type Float%20%28single-precision%29))
  (bind _asprototype_character (Utilities|Casting|CastToPrototypeCharacter (Components|GetOwner)))
  (Pawn|Input|AddMovementInput _asprototype_character (Math|Vector|GetRightVector (Math|Rotator|MakeRotator 0.0 0.0 (.Yaw (Math|Rotator|BreakRotator (Pawn|GetControlRotation _asprototype_character :!class /Script/Engine.Pawn))))) axisValue false)
  (return))