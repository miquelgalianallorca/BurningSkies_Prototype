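; Elevator Blueprint that moves a platform mesh between down and up positions when trigger volumes are overlapped.
; The platform trigger toggles direction when idle, while up and down triggers call the elevator to their level.
; Timelines drive the mesh's relative location, with DoOnce gates that re-arm when the platform overlap ends.
; A down-side collision turns on when the elevator is called down and turns off after movement finishes.
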(event OnComponentBeginOverlap(OverPlatformTrigger)
  (params (OverlappedComponent :type Primitive%20Component%20Object%20Reference) (OtherActor :type Actor%20Object%20Reference) (OtherComp :type Primitive%20Component%20Object%20Reference) (OtherBodyIndex :type Integer) (bFromSweep :type Boolean) (SweepResult :type Hit%20Result%20Structure%20%28by%20ref%29))
  (if (not (Variables|Default|GetIsMoving))
    (if (Variables|Default|GetIsUp)
      (CallFunction|GoDown)
      (else
        (CallFunction|GoUp)))))

(event OnComponentEndOverlap(OverPlatformTrigger)
  (params (OverlappedComponent :type Primitive%20Component%20Object%20Reference) (OtherActor :type Actor%20Object%20Reference) (OtherComp :type Primitive%20Component%20Object%20Reference) (OtherBodyIndex :type Integer))
  (Utilities|FlowControl|Sequence
    (:then_0
      (Utilities|FlowControl|DoOnce false) ; enters at Reset
    )
    (:then_1
      (Utilities|FlowControl|DoOnce false) ; enters at Reset
    )))

(event OnComponentBeginOverlap(UpTrigger)
  (params (OverlappedComponent :type Primitive%20Component%20Object%20Reference) (OtherActor :type Actor%20Object%20Reference) (OtherComp :type Primitive%20Component%20Object%20Reference) (OtherBodyIndex :type Integer) (bFromSweep :type Boolean) (SweepResult :type Hit%20Result%20Structure%20%28by%20ref%29))
  (if (not (Variables|Default|GetIsUp))
    (CallFunction|GoUp)))

(event OnComponentBeginOverlap(DownTrigger)
  (params (OverlappedComponent :type Primitive%20Component%20Object%20Reference) (OtherActor :type Actor%20Object%20Reference) (OtherComp :type Primitive%20Component%20Object%20Reference) (OtherBodyIndex :type Integer) (bFromSweep :type Boolean) (SweepResult :type Hit%20Result%20Structure%20%28by%20ref%29))
  (if (Variables|Default|GetIsUp)
    (Collision|SetCollisionEnabled (Variables|Default|GetDownCollision) "QueryAndPhysics")
    (CallFunction|GoDown)))

(event Custom|GoUp
  (Utilities|FlowControl|DoOnce false
    (:Completed
      (Variables|Default|SetIsMoving true)
      (bind _newtrack_1 (Timeline|Timeline_GoUp PlayFromStart)
        (:Update
          (Transformation|SetRelativeLocation (Variables|Default|GetStaticMesh) _newtrack_1 false false))
        (:Finished
          (Variables|Default|SetIsUp true)
          (Variables|Default|SetIsMoving false)
          (Collision|SetCollisionEnabled (Variables|Default|GetDownCollision) "NoCollision"))))))

(event Custom|GoDown
  (Utilities|FlowControl|DoOnce false
    (:Completed
      (Variables|Default|SetIsMoving true)
      (bind _newtrack_1 (Timeline|Timeline_GoDown ReverseFromEnd)
        (:Update
          (Transformation|SetRelativeLocation (Variables|Default|GetStaticMesh) _newtrack_1 false false))
        (:Finished
          (Variables|Default|SetIsUp false)
          (Variables|Default|SetIsMoving false)
          (Collision|SetCollisionEnabled (Variables|Default|GetDownCollision) "NoCollision"))))))

(event EventBeginPlay
  (Variables|Default|SetIsUp false)
  (Variables|Default|SetIsMoving false)
  (Collision|SetCollisionEnabled (Variables|Default|GetDownCollision) "NoCollision"))

(fn ConstructionScript)