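; BP_DynamiteTesting is a dynamite object, apparently a pickup, that spins its mesh slowly around the yaw axis every tick.
; When a PlayerCharacter overlaps its Trigger, Catch fires the OnPlayerOverlap dispatcher and hides the whole component hierarchy without destroying the actor.
; A separate Drop event deactivates the Trigger and broadcasts OnDropped, leaving visibility unchanged.
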(event OnComponentBeginOverlap(Trigger)
  (params (OverlappedComponent :type Primitive%20Component%20Object%20Reference) (OtherActor :type Actor%20Object%20Reference) (OtherComp :type Primitive%20Component%20Object%20Reference) (OtherBodyIndex :type Integer) (bFromSweep :type Boolean) (SweepResult :type Hit%20Result%20Structure%20%28by%20ref%29))
  (Utilities|Casting|CastToPlayerCharacter OtherActor)
  (CallFunction|Catch))

(event EventCatch
  (Default|CallOnPlayerOverlap)
  (Rendering|SetVisibility (Variables|Default|GetDefaultSceneRoot) false true))

(event EventTick
  (params (DeltaSeconds :type Float%20%28single-precision%29))
  (Transformation|AddLocalRotation (Variables|Default|GetDynamiteMesh3) (Math|Rotator|MakeRotator 0.0 0.0 (* DeltaSeconds 3e+01)) false false))

(event EventDrop
  (Components|Activation|Deactivate (Variables|BP_Button|GetTrigger))
  (Default|CallOnDropped))

(fn ConstructionScript)