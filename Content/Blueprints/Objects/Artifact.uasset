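; Artifact is a collectible pickup that spins continuously around its yaw axis.
; Tick rotates the Artifact component at a constant, frame-rate-independent speed.
; Its Catch event, if Hidden is false and player 0 is a PlayerCharacter, hides that component and calls OnPicked.
; The graph reads Hidden but never sets it, and only hides the component without destroying the actor.
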(event EventTick
  (params (DeltaSeconds :type Float%20%28single-precision%29))
  (Transformation|AddRelativeRotation (Variables|Default|GetArtifact) (Math|Rotator|MakeRotator 0.0 0.0 (* 1e+02 DeltaSeconds)) false false))

(event EventCatch
  (if (not (Variables|Default|GetbHidden))
    (Utilities|Casting|CastToPlayerCharacter (Game|GetPlayerCharacter 0))
    (Rendering|SetVisibility (Variables|Default|GetArtifact) false false)
    (Default|CallOnPicked)))

(fn ConstructionScript)