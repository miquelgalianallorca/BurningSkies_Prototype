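; Dynamite is a pickup object whose static mesh spins continuously around its yaw axis on Tick.
; Its Catch event runs only while Hidden is false and player 0's character casts to PlayerCharacter.
; It then hides the mesh and its children and fires the OnPicked dispatcher.
; Catch does not set Hidden or destroy the actor.
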(event EventTick
  (params (DeltaSeconds :type Float%20%28single-precision%29))
  (Transformation|AddRelativeRotation (Variables|Default|GetStaticMesh) (Math|Rotator|MakeRotator 0.0 0.0 (* 1e+02 DeltaSeconds)) false false))

(event EventCatch
  (if (not (Variables|Default|GetbHidden))
    (Utilities|Casting|CastToPlayerCharacter (Game|GetPlayerCharacter 0))
    (Rendering|SetVisibility (Variables|Default|GetStaticMesh) false true)
    (Default|CallOnPicked)))

(fn ConstructionScript)